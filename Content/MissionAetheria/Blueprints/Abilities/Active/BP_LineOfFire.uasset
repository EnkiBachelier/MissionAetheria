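; Active fire ability that turns on a flame area for a set duration, reporting burn damage on damageable actors inside it.
; Use enables box collision and a VFX visibility flag; after the duration both switch off and the ability reloads.
; Two boxes and a sphere pass overlap begin and end to a shared AI-overlap call.
; SetVFXVisibility toggles all three colliders and the Niagara fire spawn rate together.
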(event OnComponentBeginOverlap(Sphere)
  (params (OverlappedComponent :type Primitive%20Component%20Object%20Reference) (OtherActor :type Actor%20Object%20Reference) (OtherComp :type Primitive%20Component%20Object%20Reference) (OtherBodyIndex :type Integer) (bFromSweep :type Boolean) (SweepResult :type Hit%20Result%20Structure%20%28by%20ref%29))
  (bind _asidamageable (Utilities|Casting|CastToIDamageable OtherActor))
  (Default|CallOnAIOverlap true _asidamageable true (Variables|Default|GetdamageAmount)))

(event OnComponentEndOverlap(Sphere)
  (params (OverlappedComponent :type Primitive%20Component%20Object%20Reference) (OtherActor :type Actor%20Object%20Reference) (OtherComp :type Primitive%20Component%20Object%20Reference) (OtherBodyIndex :type Integer))
  (bind _asidamageable (Utilities|Casting|CastToIDamageable OtherActor))
  (Default|CallOnAIOverlap false _asidamageable true 0.0))

(event OnComponentBeginOverlap(BoxCollision)
  (params (OverlappedComponent :type Primitive%20Component%20Object%20Reference) (OtherActor :type Actor%20Object%20Reference) (OtherComp :type Primitive%20Component%20Object%20Reference) (OtherBodyIndex :type Integer) (bFromSweep :type Boolean) (SweepResult :type Hit%20Result%20Structure%20%28by%20ref%29))
  ;[1 1 1] Check object enterred collider
  (bind _asidamageable (Utilities|Casting|CastToIDamageable OtherActor))
  (Default|CallOnAIOverlap true _asidamageable true (Variables|Default|GetdamageAmount)))

(event OnComponentEndOverlap(BoxCollision)
  (params (OverlappedComponent :type Primitive%20Component%20Object%20Reference) (OtherActor :type Actor%20Object%20Reference) (OtherComp :type Primitive%20Component%20Object%20Reference) (OtherBodyIndex :type Integer))
  ;[1 1 1] Check object leave collider
  (bind _asidamageable (Utilities|Casting|CastToIDamageable OtherActor))
  (Default|CallOnAIOverlap false _asidamageable true 0.0))

(event OnComponentBeginOverlap(BoxCollision1)
  (params (OverlappedComponent :type Primitive%20Component%20Object%20Reference) (OtherActor :type Actor%20Object%20Reference) (OtherComp :type Primitive%20Component%20Object%20Reference) (OtherBodyIndex :type Integer) (bFromSweep :type Boolean) (SweepResult :type Hit%20Result%20Structure%20%28by%20ref%29))
  (bind _asidamageable (Utilities|Casting|CastToIDamageable OtherActor))
  (Default|CallOnAIOverlap true _asidamageable true (Variables|Default|GetdamageAmount)))

(event OnComponentEndOverlap(BoxCollision1)
  (params (OverlappedComponent :type Primitive%20Component%20Object%20Reference) (OtherActor :type Actor%20Object%20Reference) (OtherComp :type Primitive%20Component%20Object%20Reference) (OtherBodyIndex :type Integer))
  (bind _asidamageable (Utilities|Casting|CastToIDamageable OtherActor))
  (Default|CallOnAIOverlap false _asidamageable true 0.0))

(event Custom|OnAbilityUsed
  ;[1 1 1] When we on use of the abilities
  (CallFunction|PlayerUseAbility)
  (Default|ServerPlaySfx (Variables|Default|GetPlayerOwner) "/Game/WwiseAudio/Events/Default_Work_Unit/SFX_Character/Abilitys/Pyromaniac/Play_SFX_FLAME_MAX.Play_SFX_FLAME_MAX" (Variables|Default|GetBasePlayerController))
  (Utilities|FlowControl|Delay (Variables|Default|GetUseDuration))
  (Variables|Default|SetIsVFXVisible false)
  (Collision|SetCollisionEnabled (Variables|Default|GetBoxCollision) "NoCollision")
  (CallFunction|OnReload))

(event EventBeginPlay
  ;[1 1 1] Set abilities on start
  (CallFunction|SetVFXVisibility false)
  (Collision|SetCollisionEnabled (Variables|Default|GetBoxCollision) "NoCollision"))

(event EventEndPlay
  (params (EndPlayReason :type EEndPlayReason%20Enum :default "Destroyed"))
  (EventDispatchers|UnbindallEventsfromOnAIOverlap))

(fn ConstructionScript
  (|CallParentFunction))

(fn Use
  ;[1 1 1] When we use the abilities
  (|CallParentFunction)
  (Variables|Default|SetIsVFXVisible true)
  (Collision|SetCollisionEnabled (Variables|Default|GetBoxCollision) "QueryOnly")
  (CallFunction|OnAbilityUsed))

(fn SetVFXVisibility
  (params (ShouldbeVisible :type Boolean))
  (bind _sphere (Variables|Default|GetSphere))
  (bind _boxcollision1 (Variables|Default|GetBoxCollision1))
  (bind _boxcollision (Variables|Default|GetBoxCollision))
  (if ShouldbeVisible
    (Collision|SetCollisionEnabled _sphere "QueryOnly")
    (Collision|SetCollisionEnabled _boxcollision1 "QueryOnly")
    (Collision|SetCollisionEnabled _boxcollision "QueryOnly")
    (LocalVariables|SetSpawnRate 3e+01)
    (else
      (Collision|SetCollisionEnabled _sphere "NoCollision")
      (Collision|SetCollisionEnabled _boxcollision1 "NoCollision")
      (Collision|SetCollisionEnabled _boxcollision "NoCollision")
      (LocalVariables|SetSpawnRate 0.0)))
  (Niagara|SetNiagaraVariable(Float) (Variables|Default|GetNS_HardFire) "SpawnRate" (LocalVariables|GetSpawnRate)))