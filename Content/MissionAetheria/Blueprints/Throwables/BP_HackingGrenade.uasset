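; Throwable hacking grenade that detonates on its first overlap with a non-ignored actor and damages AI inside a short-lived vertical beam.
; Impact fires a radial impulse, sound and camera shake, hides the mesh, and spawns the Niagara beam.
; The server traces down to the named stage floor to place the beam, otherwise the actor location is used.
; A looping timer capsule-traces there to damage BP_AI actors until the grenade destroys itself.
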(event OnComponentBeginOverlap(Collision_02)
  (params (OverlappedComponent :type Primitive%20Component%20Object%20Reference) (OtherActor :type Actor%20Object%20Reference) (OtherComp :type Primitive%20Component%20Object%20Reference) (OtherBodyIndex :type Integer) (bFromSweep :type Boolean) (SweepResult :type Hit%20Result%20Structure%20%28by%20ref%29))
  (bind _returnvalue (Transformation|GetActorLocation))
  (bind (_x _y _z) (Math|Vector|BreakVector _returnvalue))
  ;[1 1 1 0.505] On collision set velocity to 0, stick the grenade where she landed and explode after X seconds
  (if (not (Utilities|Array|ContainsItem (Variables|Default|GetActorToIgnore) (Utilities|GetClass OtherActor)))
    (Collision|SetCollisionResponsetoAllChannels (Variables|Default|GetSK_HackerGrenade) "ECR_Ignore")
    (Transformation|SetWorldLocation (Variables|Default|GetSK_HackerGrenade) (Transformation|GetWorldLocation (Variables|Default|GetSK_HackerGrenade)) false false)
    (Class|RadialForceComponent|FireImpulse (Variables|Default|GetRadialForce))
    (Class|AkGameplayStatics|PostEventatLocation "/Game/WwiseAudio/Events/Default_Work_Unit/SFX_Character/Abilitys/Hacker/Play_IEM.Play_IEM" (Transformation|GetWorldLocation (Variables|Default|GetSK_HackerGrenade)) "0, 0, 0")
    (bind _outhits (Collision|MultiLineTraceByChannel _returnvalue (Math|Vector|MakeVector _x _y (- _z 1e+03)) "TraceTypeQuery1" false 0 "None"))
    (for _array_element _outhits
      (if (and (Utilities|Enum|Equal(Enum) (Utilities|GetDisplayName (.HitActor (Collision|BreakHitResult _array_element))) "SM_Stage_01_Wide_LowPoly") (Networking|IsServer))
        (Variables|Default|SetVFXLocation (.Location (Collision|BreakHitResult _array_element)))))
    (if (Utilities|Operators|EqualEqual :A (Variables|Default|GetVFXLocation))
      (Variables|Default|SetVFXLocation (Transformation|GetActorLocation)))
    (bind _returnvalue_2 (Niagara|SpawnSystematLocation "/Game/MissionAetheria/VFX/Niagara/NS_VerticalBeam.NS_VerticalBeam" (Variables|Default|GetVFXLocation) "0, 0, 0" "0.200000,0.200000,0.200000"))
    (bind _returnvalue_3 (Utilities|Time|SetTimerbyEvent (delegate Custom|Collision) 0.1 true true))
    (Class|AkGameplayStatics|PostEvent "/Game/WwiseAudio/Events/Default_Work_Unit/SFX_Character/Abilitys/Hacker/Play_IEM.Play_IEM" self)
    (CameraShake|Start (Variables|Default|GetCameraShakeExplosion))
    (Rendering|SetVisibility (Variables|Default|GetSK_HackerGrenade) false false)
    (Utilities|FlowControl|Delay 1.5)
    (Utilities|Time|ClearandInvalidateTimerbyHandle _returnvalue_3)
    (Components|DestroyComponent _returnvalue_2)
    (Actor|DestroyActor)))

(event Custom|Collision
  (bind _vfxlocation (Variables|Default|GetVFXLocation))
  ;[1 1 1 0.505] On collision set velocity to 0, stick the grenade where she landed and explode after X seconds
  (bind _outhits (Class|KismetSystemLibrary|CapsuleTraceMulti _vfxlocation _vfxlocation 1.5e+02 5e+02 "TraceTypeQuery1" false 0 "None" true))
  (for _array_element _outhits
    (if (Utilities|ClassIsChildOf (Utilities|GetClass (.hitactor _array_element)) "/Game/MissionAetheria/Blueprints/AI/BP_AI.BP_AI_C")
      (Class|IDamageable|DealDamage(Message) (.hitactor _array_element) (Variables|Default|GetAmount%20Damage) "NewEnumerator0"))))

(fn ConstructionScript)