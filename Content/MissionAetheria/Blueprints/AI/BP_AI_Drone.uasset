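; BP_AI_Drone is an AI drone character that extends a parent class and customizes only its death behavior.
; On kill, it runs the parent handler, then switches character movement to Falling and sets the capsule's constraint mode to SixDOF so the drone drops.
; BeginPlay is disabled and the construction script only calls its parent.
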(event EventBeginPlay
  (|CallParentFunction) ; This node is disabled and will not be called.\nDrag off pins to build functionality.
)

(fn ConstructionScript
  (|CallParentFunction))

(fn OnKilled
  (|CallParentFunction)
  (Pawn|Components|CharacterMovement|SetMovementMode (Variables|Character|GetCharacterMovement) "MOVE_Falling" 0)
  (Class|PrimitiveComponent|SetConstraintMode (Variables|Default|GetCapsuleComponent) "SixDOF"))