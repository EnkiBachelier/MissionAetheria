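; BP_Minigun is a hitscan minigun weapon that extends a parent weapon Blueprint.
; ShootBullet plays Wwise fire audio and muzzle VFX through server calls, then line-traces from the pawn's camera and sends damage on any IDamageable hit via the player controller.
; Reload adds server-played audio, and SetMuzzleShotVFXVisibility toggles the MuzzleShot effect, which is also requested off at BeginPlay.
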(event Custom|OnWeaponUsed)

(event EventBeginPlay
  (Default|ServerShowMuzzleShotVFX (CallFunction|GetBasePlayerController) "NewEnumerator0" false)
  (|CallParentFunction))

(fn ConstructionScript
  (|CallParentFunction))

(fn ShootBullet
  (|CallParentFunction)
  (Default|ServerPlaySfx (Variables|Default|GetPlayerOwner) "/Game/WwiseAudio/Events/Default_Work_Unit/SFX_Character/Pilot/Play_SFX_War_plane_minigun.Play_SFX_War_plane_minigun" (Variables|Default|GetBasePlayerController))
  (Default|ServerShowMuzzleShotVFX (CallFunction|GetBasePlayerController) "NewEnumerator0" true)
  (bind _outhit (Default|CameraLineTrace (Default|GetPlayerPawn (CallFunction|GetBasePlayerController)) (Variables|Default|GetMaxBulletDistance)))
  (bind _asidamageable (Utilities|Casting|CastToIDamageable (.hitactor _outhit)))
  (Default|ServerDealDamage (CallFunction|GetBasePlayerController) (Variables|Default|GetAmountDamage) _asidamageable false false (Variables|Default|GetPlayerOwner)))

(fn SetMuzzleShotVFXVisibility
  (params (IsActive :type Boolean))
  (bind _muzzleshot (Variables|Default|GetMuzzleShot))
  (if IsActive
    (Components|Activation|Activate _muzzleshot true)
    (else
      (Components|Activation|Deactivate _muzzleshot)))
  (|CallParentFunction false))

(fn Reload
  (|CallParentFunction)
  (Default|ServerPlaySfx (Variables|Default|GetPlayerOwner) "/Game/WwiseAudio/Events/Default_Work_Unit/SFX_Character/Weapons/Pilot/Play_SFX_reloading_minigun.Play_SFX_reloading_minigun" (Variables|Default|GetBasePlayerController)))