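; Medic active ability that turns pistol damage into self-healing for a limited time.
; Init binds to the pistol's entity-damaged event; while active and below max life, each hit heals by damage times an energy multiplier and shows VFX, both through server calls on the character.
; Use activates it, then OnReload waits out the duration, deactivates it and runs the parent reload.
; Owner and Medic references are lazily cast and cached.
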(event Custom|OnEntityDamaged
  (params (DamageAmount :type Float%20%28double-precision%29))
  (bind _base_playable_character (CallFunction|GetBasePlayableCharacter))
  ;[1 1 1] On Entity Damaged
  (if (Variables|Default|GetIsAbilityActive)
    (if (< (Variables|/Game/MissionAetheria/Blueprints/Player/BP_BasePlayableCharacter.BP_BasePlayableCharacter_C|GetCurrentHP _base_playable_character) (.maxlife (Variables|/Game/MissionAetheria/Blueprints/Player/BP_BasePlayableCharacter.BP_BasePlayableCharacter_C|GetCharacterDatas _base_playable_character)))
      (Default|ServerSetCurrentHp (CallFunction|GetBasePlayableCharacter) (+ (Variables|/Game/MissionAetheria/Blueprints/Player/BP_BasePlayableCharacter.BP_BasePlayableCharacter_C|GetCurrentHP (CallFunction|GetBasePlayableCharacter)) (* DamageAmount (Variables|Default|GetEnergyMultiplier))) "NewEnumerator5")
      (Default|ServerShowMedicVFXAbility (CallFunction|GetMedic)))))

(event EventBeginPlay)

(event EventOnReload
  ;[1 1 1] On Reload
  (Utilities|FlowControl|Delay (Variables|Default|GetUseDuration)) ; Duration of the ability
  (Variables|Default|SetIsAbilityActive false)
  (|CallParentFunction))

(fn ConstructionScript
  (|CallParentFunction))

(fn Use
  (Variables|Default|SetIsAbilityActive true)
  (CallFunction|PlayerUseAbility)
  (|CallParentFunction)
  (CallFunction|OnReload))

(fn Init
  (params (Pistol :type BP%20Pistol%20Object%20Reference))
  (EventDispatchers|BindEventtoOnEntityDamaged Pistol (EventDispatchers|CreateEvent :!event Custom|OnEntityDamaged)))

(fn GetBasePlayableCharacter
  (Variables|Default|GetBase%20Playable%20Character
    (:then
      (return (Variables|Default|GetBase%20Playable%20Character)))
    (:else
      (bind _asbp_base_playable_character (Utilities|Casting|CastToBP_BasePlayableCharacter (Actor|GetParentActor))
        (:then
          (Variables|Default|SetBase%20Playable%20Character _asbp_base_playable_character)
          (return (Variables|Default|GetBase%20Playable%20Character)))
        (:CastFailed
          (Development|PrintString "BP_Medic | Cast to PC_BasePlayableCharacter failed !"))))))

(fn SetVFXVisibility
  (params (ShouldbeVisible :type Boolean))
  (Niagara|SpawnSystematLocation 0 "0, 0, 0"))

(fn GetMedic
  (Variables|Default|GetPlayerMedic
    (:then
      _)
    (:else
      (bind _asbp_playable_character_medic (Utilities|Casting|CastToBP_PlayableCharacter_Medic (CallFunction|GetBasePlayableCharacter)))
      (Variables|Default|SetPlayerMedic _asbp_playable_character_medic)))
  (return (Variables|Default|GetPlayerMedic)))