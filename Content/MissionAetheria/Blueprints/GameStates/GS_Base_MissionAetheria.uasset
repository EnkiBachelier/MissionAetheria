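; Base game state for Mission Aetheria, holding the player list and handling music, level switches and wave records.
; On BeginPlay it starts music through a lazily spawned Wwise music manager and rebuilds Players from the game instance's role choices.
; A cached game instance getter serves level switching and analytics.
; Wave records pass from a server event to a multicast that updates each game instance's survival record.
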(event Custom|Client_OnSwitchLevel
  (params (newLevelName :type String))
  (Default|SwitchLevel (CallFunction|GetGameInstance) newLevelName))

(event Custom|Server_SaveWaveRecord
  (params (WavesSurvivedRecordToAdd :type Float%20%28double-precision%29))
  (CallFunction|MulticastSaveWaveRecord WavesSurvivedRecordToAdd))

(event Custom|Multicast_SaveWaveRecord
  (params (WavesSurvivedRecordToAdd :type Float%20%28double-precision%29))
  (bind _gameinstance (CallFunction|GetGameInstance))
  (bind _analytics (Variables|/Game/MissionAetheria/Blueprints/GameInstance/GI_MissionAetheria.GI_MissionAetheria_C|GetAnalytics _gameinstance))
  (Utilities|IsValid _analytics
    (:Is%20Valid
      (Default|UpdateWavesSurvivedRecord _analytics WavesSurvivedRecordToAdd))
    (:Is%20Not%20Valid
      (Development|PrintString "Failed to Find GAme instance analytics" false))))

(event EventBeginPlay
  (CallFunction|HandleMusic (Variables|Default|GetMusicState) "NewEnumerator4")
  (if (> (Utilities|Array|Length (Variables|/Game/MissionAetheria/Blueprints/GameInstance/GI_MissionAetheria.GI_MissionAetheria_C|GetPlayersRoleChoice (CallFunction|GetGameInstance))) 0)
    (Utilities|Array|Clear (Variables|Default|GetPlayers))
    (for _array_element (Variables|/Game/MissionAetheria/Blueprints/GameInstance/GI_MissionAetheria.GI_MissionAetheria_C|GetPlayersRoleChoice (CallFunction|GetGameInstance))
      (Utilities|Array|AddUnique (Variables|Default|GetPlayers) (.player _array_element)))))

(event EventTick
  (params (DeltaSeconds :type Float%20%28single-precision%29)))

(fn ConstructionScript)

(fn AddPlayer
  (params (player :type Struct%20Player%20Structure%20%28by%20ref%29))
  (if (Utilities|Enum|NotEqual(Enum) (Utilities|String|ToString(Name) (.Name (Utilities|Struct|BreakStruct_Player player))) "None")
    (Utilities|Array|AddUnique (Variables|Default|GetPlayers) player)))

(fn GetGameInstance
  (Utilities|IsValid (Variables|Default|GetGameInstance)
    (:Is%20Valid
      _)
    (:Is%20Not%20Valid
      (bind _asgi_mission_aetheria (Utilities|Casting|CastToGI_MissionAetheria (Game|GetGameInstance)))
      (Variables|Default|SetGameInstance _asgi_mission_aetheria)))
  (return (Variables|Default|GetGameInstance)))

(fn HandleMusic
  (params (MusicState :type Enum_MusicState%20Enum :default "NewEnumerator0") (BattleState :type BattleState%20Enum :default "NewEnumerator0"))
  (if (Utilities|IsValid (Variables|Default|GetMusicManagerRef))
    (Default|PlayMusic (Variables|Default|GetMusicManagerRef) MusicState BattleState false)
    (else
      (bind _returnvalue (Game|SpawnActorfromClass "/Game/MissionAetheria/Blueprints/Sounds/BP_WwiseMusicManager.BP_WwiseMusicManager_C" (Math|Transform|MakeTransform "0, 0, 0") "Undefined" "MultiplyWithRoot" 0 0))
      (bind _output_get (Variables|Default|SetMusicManagerRef _returnvalue))
      (Default|PlayMusic _output_get MusicState BattleState false))))