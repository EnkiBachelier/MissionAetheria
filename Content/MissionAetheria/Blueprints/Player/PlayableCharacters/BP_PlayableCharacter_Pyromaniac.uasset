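; Playable Pyromaniac character, a child of a base character class, that carries a flamethrower as a child actor.
; On BeginPlay it sets its character data, runs parent setup, registers three cannisters and hands itself to the flamethrower as owning Pyromaniac.
; A server event relays flamethrower VFX visibility to all clients through a multicast.
; GetFlamethrower lazily casts and caches the child actor, with Valid and NotValid exits.
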(event Custom|Server_FlamethrowerVisibility
  (params (ShouldBeVisble :type Boolean))
  ;[1 1 1] Set Flamethrower Visibility
  (CallFunction|MulticastFlamethrowerVisibility ShouldBeVisble))

(event Custom|Multicast_FlamethrowerVisibility
  (params (ShouldBeVisible :type Boolean))
  ;[1 1 1] Set Flamethrower Visibility
  (bind _flamethrower (Utilities|GetFlamethrower)
    (:Valid
      (Default|SetVFXVisibilty _flamethrower ShouldBeVisible))))

(event EventBeginPlay
  (CallFunction|SetData "NewEnumerator2")
  (|CallParentFunction)
  (for _array_element (Utilities|Array|MakeArray (Variables|Default|GetCan_0) (Variables|Default|GetCan_1) (Variables|Default|GetCan_2))
    (CallFunction|AddCannistertotheArray _array_element)
    (bind _flamethrower (Utilities|GetFlamethrower)
      (:Valid
        (Variables|/Game/MissionAetheria/Blueprints/Weapons/BP_Flamethrower.BP_Flamethrower_C|SetPyromaniac _flamethrower self)))))

(fn ConstructionScript
  (|CallParentFunction))