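; BP_Flamethrower is the Pyromaniac's flamethrower weapon, applying burn damage to damageable actors in its flame area.
; Box and sphere overlaps report targets entering or leaving to the parent's AI overlap call.
; Shoot, release and reload toggle a RepNotify visibility flag, forwarded to the Pyromaniac through a server call, while shooting and reloading play Wwise sounds.
; SetVFXVisibilty switches the Niagara spawn rate and both damage colliders together.
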(event OnComponentBeginOverlap(Sphere)
  (params (OverlappedComponent :type Primitive%20Component%20Object%20Reference) (OtherActor :type Actor%20Object%20Reference) (OtherComp :type Primitive%20Component%20Object%20Reference) (OtherBodyIndex :type Integer) (bFromSweep :type Boolean) (SweepResult :type Hit%20Result%20Structure%20%28by%20ref%29))
  (bind _asidamageable (Utilities|Casting|CastToIDamageable OtherActor))
  (Default|CallOnAIOverlap true _asidamageable true (Variables|Default|GetAmountDamage)))

(event OnComponentEndOverlap(Sphere)
  (params (OverlappedComponent :type Primitive%20Component%20Object%20Reference) (OtherActor :type Actor%20Object%20Reference) (OtherComp :type Primitive%20Component%20Object%20Reference) (OtherBodyIndex :type Integer))
  (bind _asidamageable (Utilities|Casting|CastToIDamageable OtherActor))
  (Default|CallOnAIOverlap false _asidamageable true 0.0))

(event OnComponentBeginOverlap(BoxCollision)
  (params (OverlappedComponent :type Primitive%20Component%20Object%20Reference) (OtherActor :type Actor%20Object%20Reference) (OtherComp :type Primitive%20Component%20Object%20Reference) (OtherBodyIndex :type Integer) (bFromSweep :type Boolean) (SweepResult :type Hit%20Result%20Structure%20%28by%20ref%29))
  ;[1 1 1] Check object entered collider
  (bind _asidamageable (Utilities|Casting|CastToIDamageable OtherActor))
  (Default|CallOnAIOverlap true _asidamageable true (Variables|Default|GetAmountDamage)))

(event OnComponentEndOverlap(BoxCollision)
  (params (OverlappedComponent :type Primitive%20Component%20Object%20Reference) (OtherActor :type Actor%20Object%20Reference) (OtherComp :type Primitive%20Component%20Object%20Reference) (OtherBodyIndex :type Integer))
  ;[1 1 1] Check object leave collider
  (bind _asidamageable (Utilities|Casting|CastToIDamageable OtherActor))
  (Default|CallOnAIOverlap false _asidamageable true 0.0))

(event EventBeginPlay
  (CallFunction|SetVFXVisibilty false)
  (|CallParentFunction))

(fn ConstructionScript
  (|CallParentFunction))

(fn ShootBullet
  ;[1 1 1] What we'll do the bullet when shoot
  (|CallParentFunction)
  (Default|ServerPlaySfx (Variables|Default|GetPlayerOwner) "/Game/WwiseAudio/Events/Default_Work_Unit/SFX_Character/Weapons/Pyromaniac/Play_SFX_FLAME.Play_SFX_FLAME" (Variables|Default|GetBasePlayerController))
  (if (not (Variables|Default|GetIsVFXVisible))
    (Variables|Default|SetIsVFXVisible true)))

(fn Reload
  ;[1 1 1] When we are on reload
  (Default|ServerPlaySfx (Variables|Default|GetPlayerOwner) "/Game/WwiseAudio/Events/Default_Work_Unit/SFX_Character/Weapons/Pyromaniac/Play_SFX_FLAME_RELOAD.Play_SFX_FLAME_RELOAD" (Variables|Default|GetBasePlayerController))
  (CallFunction|SetVFXVisibilty false)
  (Variables|Default|SetIsVFXVisible false)
  (|CallParentFunction))

(fn ReleaseShootInput
  ;[1 1 1] When we stop shooting with the weapon
  (Variables|Default|SetIsVFXVisible false))

(fn SetVFXVisibilty
  (params (shouldBeVisible :type Boolean))
  (bind _boxcollision (Variables|Default|GetBoxCollision))
  (bind _sphere (Variables|Default|GetSphere))
  (if shouldBeVisible
    (LocalVariables|SetspawnRate 3e+01)
    (Collision|SetCollisionEnabled _boxcollision "QueryOnly")
    (Collision|SetCollisionEnabled _sphere "QueryOnly")
    (else
      (LocalVariables|SetspawnRate 0.0)
      (Collision|SetCollisionEnabled _boxcollision "NoCollision")
      (Collision|SetCollisionEnabled _sphere "NoCollision")))
  (Niagara|SetNiagaraVariable(Float) (Variables|Default|GetNS_SoftFire) "SpawnRate" (LocalVariables|GetspawnRate)))

(fn OnRepPlayerOwner
  (Variables|Default|SetIsVFXVisible false))

(fn OnRepIsVFXVisible
  (Default|ServerFlamethrowerVisibility (CallFunction|GetPyromaniac) (Variables|Default|GetIsVFXVisible)))

(fn GetPyromaniac
  (Variables|Default|GetPyromaniac
    (:then
      _)
    (:else
      (bind _playerowner (Variables|Default|GetPlayerOwner)
        (:then
          (bind _asbp_playable_character_pyromaniac (Utilities|Casting|CastToBP_PlayableCharacter_Pyromaniac _playerowner))
          (Variables|Default|SetPyromaniac _asbp_playable_character_pyromaniac))
        (:else))))
  (return (Variables|Default|GetPyromaniac)))