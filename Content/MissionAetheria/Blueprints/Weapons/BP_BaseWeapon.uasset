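; Base weapon Blueprint that handles firing, ammo and reloading for its owning player, with bullet behavior left to child classes.
; TryToFire routes to delay-driven OnFire or OnReload events, using state flags to pace shots and block fire during reloads.
; Reloading refills ammo and toggles the stage widget's animation.
; BoostWeaponData modifies reload time, shot delay or magazine size, with the shot-delay boost non-stacking and restored from its cached default.
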(event Custom|OnFire
  ;[0.05781 0.05781 0.05781] OnFire
  (if (not (Variables|Default|GetIsShooting))
    (Variables|Default|SetIsShooting true)
    (Math|Integer|DecrementInt (Variables|Default|GetCurrentBulletCount)
      (:%20%20
        (CallFunction|ShootBullet)
        (Utilities|FlowControl|Delay (.DelayBetweenEachShot (Utilities|Struct|BreakStruct_WeaponData (Variables|Default|GetWeaponData))))
        (Variables|Default|SetIsShooting false)))))

(event Custom|OnReload
  ;[0.05781 0.05781 0.05781] OnReload
  (bind _output_get (Variables|Default|SetIsReloading true))
  (CallFunction|Reload)
  (CallFunction|ShowReloadingAnim _output_get)
  (Utilities|FlowControl|Delay (.ReloadDuration (Utilities|Struct|BreakStruct_WeaponData (Variables|Default|GetWeaponData))))
  (bind _output_get_2 (Variables|Default|SetIsReloading false))
  (CallFunction|ShowReloadingAnim _output_get_2))

(event EventBeginPlay
  (bind _weapondata (Variables|Default|GetWeaponData))
  (bind (_reloadduration _delaybetweeneachshot _maxbulletcount) (Utilities|Struct|BreakStruct_WeaponData _weapondata))
  ;[0.05781 0.05781 0.05781] BeginPlay
  (Variables|Default|SetCurrentBulletCount _maxbulletcount)
  (Variables|Default|SetDefault%20Delay%20Between%20Each%20Shot _delaybetweeneachshot))

(event EventDestroyed
  (EventDispatchers|UnbindallEventsfromOnAIOverlap))

(fn ConstructionScript)

(fn TrytoFire
  (if (<= (Variables|Default|GetCurrentBulletCount) 0)
    (CallFunction|OnReload)
    (elif (not (Variables|Default|GetIsReloading))
      (CallFunction|OnFire))))

(fn Reload
  (Variables|Default|SetCurrentBulletCount (.MaxBulletCount (Utilities|Struct|BreakStruct_WeaponData (Variables|Default|GetWeaponData)))))

(fn ShootBullet
  (bind _playerowner (Variables|Default|GetPlayerOwner)
    (:then
      (Default|ShootAction _playerowner))
    (:else)))

(fn ReleaseShootInput)

(fn BoostWeaponData
  (params (DataTypeToModify :type Enum_WeaponDataType%20Enum :default "NewEnumerator0") (Multiplier :type Float%20%28double-precision%29) (ShouldDivide :type Boolean) (IsEnd :type Boolean))
  (switch Utilities|FlowControl|Switch|SwitchonEnum_WeaponDataType DataTypeToModify
    (:NewEnumerator0
      (Utilities|BoostReloadTime Multiplier ShouldDivide))
    (:NewEnumerator1
      (if IsEnd
        (CallFunction|RemoveBoostDelayBetweenShots)
        (else
          (CallFunction|StartBoostDelayBetweenShots Multiplier))))
    (:NewEnumerator2
      (Utilities|BoostMaxBulletCount Multiplier ShouldDivide))))

(fn OnRepIsShooting
  (Default|CallOnSetIsShooting))

(fn OnRepIsReloading
  (Default|CallOnSetIsReloading))

(fn SetMuzzleShotVFXVisibility
  (params (IsActive :type Boolean)))

(fn GetBasePlayerController
  (Variables|Default|GetBasePlayerController
    (:then
      _)
    (:else
      (bind _aspc_base_player_controller (Utilities|Casting|CastToPC_BasePlayerController (Game|GetPlayerController 0)))
      (Variables|Default|SetBasePlayerController _aspc_base_player_controller)))
  (return (Variables|Default|GetBasePlayerController)))

(fn RemoveBoostDelayBetweenShots
  (Variables|Default|SetWeaponData (Utilities|Struct|MakeStruct_WeaponData (.reloadduration (Variables|Default|GetWeaponData)) (Variables|Default|GetDefault%20Delay%20Between%20Each%20Shot) (.maxbulletcount (Variables|Default|GetWeaponData))))
  (Variables|Default|SetAsBoostDelayBetweenShots false))

(fn StartBoostDelayBetweenShots
  (params (Multiplier :type Float%20%28double-precision%29))
  (if (not (Variables|Default|GetAsBoostDelayBetweenShots))
    (Variables|Default|SetWeaponData (Utilities|Struct|MakeStruct_WeaponData (.reloadduration (Variables|Default|GetWeaponData)) (/ (.delaybetweeneachshot (Variables|Default|GetWeaponData)) Multiplier) (.maxbulletcount (Variables|Default|GetWeaponData))))
    (Variables|Default|SetAsBoostDelayBetweenShots true)))

(fn ShowReloadingAnim
  (params (Show :type Boolean))
  (Default|ShowReloadingAnimation (Variables|/Game/MissionAetheria/Blueprints/PlayerControllers/PC_BasePlayerController.PC_BasePlayerController_C|GetWBPStageGeneral (Default|GetPlayerController (Variables|Default|GetPlayerOwner))) Show))