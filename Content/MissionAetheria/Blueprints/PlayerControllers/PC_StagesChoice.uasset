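; Player controller for the stage choice screen, spawning the local player and relaying lobby actions to the server.
; On BeginPlay it asks the server to spawn the game instance's current player through GM_StagesChoice and sets game-only input.
; Server events forward level switches to GS_StagesChoice and flip a slot panel's front-view flag.
; Game mode, game instance and game state getters lazily cast and cache their references.
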(event Custom|ServerTurnPanel
  (params (isFront :type Boolean) (slot :type BP%20Slot%20Object%20Reference))
  (Variables|/Game/MissionAetheria/Blueprints/StagesChoice/InteractableObject/Slots/BP_Slot.BP_Slot_C|SetisPanelViewFront slot isFront))

(event Custom|Server_SwitchLevel
  (params (newLevelName :type String))
  ;[0.03125 0.03125 0.03125] SwitchLevel
  (Default|ClientonSwitchLevel (CallFunction|GetGameState) newLevelName))

(event Custom|Server_SpawnPlayer
  (params (player :type Struct%20Player%20Structure))
  (Default|SpawnPlayer (CallFunction|GetGameMode) self player))

(event EventBeginPlay
  (if (Pawn|IsLocalPlayerController)
    (CallFunction|ServerSpawnPlayer (Variables|/Game/MissionAetheria/Blueprints/GameInstance/GI_MissionAetheria.GI_MissionAetheria_C|GetCurrentPlayer (CallFunction|GetGameInstance)))
    (Input|SetInputModeGameOnly self false)))

(fn ConstructionScript)

(fn GetGameMode
  (Variables|Default|GetGameMode
    (:then
      _)
    (:else
      (bind _asgm_stages_choice (Utilities|Casting|CastToGM_StagesChoice (Game|GetGameMode)))
      (Variables|Default|SetGameMode _asgm_stages_choice)))
  (return (Variables|Default|GetGameMode)))

(fn GetGameInstance
  (Variables|Default|GetGameInstance
    (:then
      _)
    (:else
      (bind _asgi_mission_aetheria (Utilities|Casting|CastToGI_MissionAetheria (Game|GetGameInstance)))
      (Variables|Default|SetGameInstance _asgi_mission_aetheria)))
  (return (Variables|Default|GetGameInstance)))

(fn GetGameState
  (Utilities|IsValid (Variables|Default|GetGameState)
    (:Is%20Valid
      _)
    (:Is%20Not%20Valid
      (bind _asgs_stages_choice (Utilities|Casting|CastToGS_StagesChoice (Game|GetGameState)))
      (Variables|Default|SetGameState _asgs_stages_choice)))
  (return (Variables|Default|GetGameState)))