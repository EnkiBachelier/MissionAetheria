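; BP_Analytics records player statistics (games, wins, losses, time played, character usage, connection dates, best waves survived) in Firebase documents under Users/<player ID>.
; The player ID comes from the local FirebaseData save game.
; InitDocuments rewrites the document with defaults for missing fields, then refreshes the last connection date.
; Each public function fetches the document, and per-stat callbacks increment, overwrite or raise the value before writing it back.
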(event Custom|INIT%20On%20Update%20Document%20Fail
  (params (Message :type String))
  ;[1 1 1] On Update Document
  (Development|PrintString 0 (Utilities|String|Append "Error when initializing document : " Message) false true "(R=1.000000,G=0.000000,B=0.028754,A=1.000000)" 5.0))

(event Custom|INIT%20On%20Load%20Document%20Fail
  (params (DocumentId :type String))
  ;[1 1 1] On Load Document
  (Development|PrintString 0 (Utilities|String|Append "Failed to load document : " DocumentId) false true "(R=1.000000,G=0.008761,B=0.000000,A=1.000000)"))

(event Custom|INIT%20On%20Update%20Document%20Success
  (params (Message :type String))
  ;[1 1 1] On Update Document
  (Development|PrintString 0 "Succesfuly initalized document" false true "(R=0.204539,G=1.000000,B=0.000000,A=1.000000)" 5.0)
  (LastConnectionDate|UpdateLastConnectionDate))

(event Custom|INIT%20On%20Load%20Document%20Success
  (params (DocumentId :type String) (DocumentSnapshot :type Document%20Snapshot%20Structure))
  ;[1 1 1] On Load Document
  (bind _returnvalue (Class|FBPDataObject|FBPBeginWriteDocument))
  (bind _updated_document (General|GetAllDocument DocumentSnapshot _returnvalue))
  (bind _player_id (Utilities|GetFireBaseSaveData)
    (:Success
      (Class|FBPFirestore|FBPAddDocument (Utilities|Array|MakeArray "Users" _player_id) _updated_document (EventDispatchers|CreateEvent :!event Custom|INIT%20On%20Update%20Document%20Success) (EventDispatchers|CreateEvent :!event Custom|INIT%20On%20Update%20Document%20Fail)))))

(event Custom|GPC%20On%20Load%20Document%20Fail
  (params (Document%20ID :type String))
  ;[1 1 1] On Load Document
  (Development|PrintString 0 (Utilities|String|Append "Error when loading document : " Document%20ID) false true "(R=1.000000,G=0.000000,B=0.037924,A=1.000000)" 5.0))

(event Custom|GPC%20On%20Update%20Document%20Fail
  (params (Document%20ID :type String))
  ;[1 1 1] On Update Document
  (Development|PrintString 0 (Utilities|String|Append "Error when adding document : " Document%20ID) false true "(R=1.000000,G=0.000000,B=0.037924,A=1.000000)" 5.0))

(event Custom|GPC%20On%20Load%20Document%20Success
  (params (Document%20ID :type String) (Document%20Snapshot :type Document%20Snapshot%20Structure))
  ;[1 1 1] On Load Document
  (bind _returnvalue (Class|FBPDataObject|FBPBeginWriteDocument))
  (bind _returnvalue_2 (Class|FBPDataObject|GetNumber (Variables|Keys|GetKey%20GamePlayedCount) Document%20Snapshot))
  (bind _returnvalue_3 (Class|FBPDataObject|AddNumber (Variables|Keys|GetKey%20GamePlayedCount) (+ _returnvalue_2 1.0) _returnvalue))
  (bind _player_id (Utilities|GetFireBaseSaveData)
    (:Success
      (Class|FBPFirestore|FBPUpdateDocument (Utilities|Array|MakeArray "Users" _player_id) _returnvalue_3 (EventDispatchers|CreateEvent :!event Custom|GPC%20On%20Update%20Document%20Success) (EventDispatchers|CreateEvent :!event Custom|GPC%20On%20Update%20Document%20Fail)))))

(event Custom|GPC%20On%20Update%20Document%20Success
  (params (Document%20ID :type String))
  ;[1 1 1] On Update Document
  (Development|PrintString 0 (Utilities|String|Append "Document " Document%20ID "added succesfuly") false true "(R=0.000000,G=1.000000,B=0.047720,A=1.000000)" 5.0))

(event Custom|GWC%20On%20Load%20Document%20Fail
  (params (Document%20ID :type String))
  ;[1 1 1] On Load Document
  (Development|PrintString 0 (Utilities|String|Append "Error when loading document : " Document%20ID) false true "(R=1.000000,G=0.000000,B=0.037924,A=1.000000)" 5.0))

(event Custom|GWC%20On%20Update%20Document%20Fail
  (params (Document%20ID :type String))
  ;[1 1 1] On Update Document
  (Development|PrintString 0 (Utilities|String|Append "Error when adding document : " Document%20ID) false true "(R=1.000000,G=0.000000,B=0.037924,A=1.000000)" 5.0))

(event Custom|GWC%20On%20Load%20Document%20Success
  (params (Document%20ID :type String) (Document%20Snapshot :type Document%20Snapshot%20Structure))
  ;[1 1 1] On Load Document
  (bind _returnvalue (Class|FBPDataObject|FBPBeginWriteDocument))
  (bind _returnvalue_2 (Class|FBPDataObject|GetNumber (Variables|Keys|GetKey%20Wins) Document%20Snapshot))
  (bind _returnvalue_3 (Class|FBPDataObject|AddNumber (Variables|Keys|GetKey%20Wins) (+ _returnvalue_2 1.0) _returnvalue))
  (bind _player_id (Utilities|GetFireBaseSaveData)
    (:Success
      (Class|FBPFirestore|FBPUpdateDocument (Utilities|Array|MakeArray "Users" _player_id) _returnvalue_3 (EventDispatchers|CreateEvent :!event Custom|GWC%20On%20Update%20Document%20Success) (EventDispatchers|CreateEvent :!event Custom|GWC%20On%20Update%20Document%20Fail)))))

(event Custom|GWC%20On%20Update%20Document%20Success
  (params (Document%20ID :type String))
  ;[1 1 1] On Update Document
  (Development|PrintString 0 (Utilities|String|Append "Document " Document%20ID "added succesfuly") false true "(R=0.000000,G=1.000000,B=0.047720,A=1.000000)" 5.0))

(event Custom|GLC%20On%20Load%20Document%20Fail
  (params (Document%20ID :type String))
  ;[1 1 1] On Load Document
  (Development|PrintString 0 (Utilities|String|Append "Error when loading document : " Document%20ID) false true "(R=1.000000,G=0.000000,B=0.037924,A=1.000000)" 5.0))

(event Custom|GLC%20On%20Update%20Document%20Fail
  (params (Document%20ID :type String))
  ;[1 1 1] On Update Document
  (Development|PrintString 0 (Utilities|String|Append "Error when adding document : " Document%20ID) false true "(R=1.000000,G=0.000000,B=0.037924,A=1.000000)" 5.0))

(event Custom|GLC%20On%20Load%20Document%20Success
  (params (Document%20ID :type String) (Document%20Snapshot :type Document%20Snapshot%20Structure))
  ;[1 1 1] On Load Document
  (bind _returnvalue (Class|FBPDataObject|FBPBeginWriteDocument))
  (bind _returnvalue_2 (Class|FBPDataObject|GetNumber (Variables|Keys|GetKey%20Loses) Document%20Snapshot))
  (bind _returnvalue_3 (Class|FBPDataObject|AddNumber (Variables|Keys|GetKey%20Loses) (+ _returnvalue_2 1.0) _returnvalue))
  (bind _player_id (Utilities|GetFireBaseSaveData)
    (:Success
      (Class|FBPFirestore|FBPUpdateDocument (Utilities|Array|MakeArray "Users" _player_id) _returnvalue_3 (EventDispatchers|CreateEvent :!event Custom|GLC%20On%20Update%20Document%20Success) (EventDispatchers|CreateEvent :!event Custom|GLC%20On%20Update%20Document%20Fail)))))

(event Custom|GLC%20On%20Update%20Document%20Success
  (params (Document%20ID :type String))
  ;[1 1 1] On Update Document
  (Development|PrintString 0 (Utilities|String|Append "Document " Document%20ID "added succesfuly") false true "(R=0.000000,G=1.000000,B=0.047720,A=1.000000)" 5.0))

(event Custom|UTP%20On%20Load%20Document%20Fail
  (params (Document%20ID :type String))
  ;[1 1 1] On Load Document
  (Development|PrintString 0 (Utilities|String|Append "Error when loading document : " Document%20ID) false true "(R=1.000000,G=0.000000,B=0.037924,A=1.000000)" 5.0))

(event Custom|UTP%20On%20Update%20Document%20Fail
  (params (Document%20ID :type String))
  ;[1 1 1] On Update Document
  (Development|PrintString 0 (Utilities|String|Append "Error when adding document : " Document%20ID) false true "(R=1.000000,G=0.000000,B=0.037924,A=1.000000)" 5.0))

(event Custom|UTP%20On%20Load%20Document%20Success
  (params (Document%20ID :type String) (Document%20Snapshot :type Document%20Snapshot%20Structure))
  ;[1 1 1] On Load Document
  (bind _returnvalue (Class|FBPDataObject|FBPBeginWriteDocument))
  (bind _returnvalue_2 (Class|FBPDataObject|GetNumber (Variables|Keys|GetKey%20TimePlayed) Document%20Snapshot))
  (bind _returnvalue_3 (Class|FBPDataObject|AddNumber (Variables|Keys|GetKey%20TimePlayed) (+ _returnvalue_2 (Variables|Values|GetTimePlayedValueToAdd)) _returnvalue))
  (bind _player_id (Utilities|GetFireBaseSaveData)
    (:Success
      (Class|FBPFirestore|FBPUpdateDocument (Utilities|Array|MakeArray "Users" _player_id) _returnvalue_3 (EventDispatchers|CreateEvent :!event Custom|UTP%20On%20Update%20Document%20Success) (EventDispatchers|CreateEvent :!event Custom|UTP%20On%20Update%20Document%20Fail)))))

(event Custom|UTP%20On%20Update%20Document%20Success
  (params (Document%20ID :type String))
  ;[1 1 1] On Update Document
  (Development|PrintString 0 (Utilities|String|Append "Document " Document%20ID "added succesfuly") false true "(R=0.000000,G=1.000000,B=0.047720,A=1.000000)" 5.0))

(event Custom|CTUHT%20On%20Load%20Document%20Fail
  (params (Document%20ID :type String))
  ;[1 1 1] On Load Document
  (Development|PrintString 0 (Utilities|String|Append "Error when loading document : " Document%20ID) false true "(R=1.000000,G=0.000000,B=0.037924,A=1.000000)" 5.0))

(event Custom|CTUHT%20On%20Update%20Document%20Fail
  (params (Document%20ID :type String))
  ;[1 1 1] On Update Document
  (Development|PrintString 0 (Utilities|String|Append "Error when adding document : " Document%20ID) false true "(R=1.000000,G=0.000000,B=0.037924,A=1.000000)" 5.0))

(event Custom|CTUHT%20On%20Load%20Document%20Success
  (params (Document%20ID :type String) (Document%20Snapshot :type Document%20Snapshot%20Structure))
  ;[1 1 1] On Load Document
  (bind _returnvalue (Class|FBPDataObject|FBPBeginWriteDocument))
  (bind _returnvalue_2 (Class|FBPDataObject|GetNumber (Variables|Keys|GetKey%20TimeUsedHackerTank) Document%20Snapshot))
  (bind _returnvalue_3 (Class|FBPDataObject|AddNumber (Variables|Keys|GetKey%20TimeUsedHackerTank) (+ _returnvalue_2 1.0) _returnvalue))
  (bind _player_id (Utilities|GetFireBaseSaveData)
    (:Success
      (Class|FBPFirestore|FBPUpdateDocument (Utilities|Array|MakeArray "Users" _player_id) _returnvalue_3 (EventDispatchers|CreateEvent :!event Custom|CTUHT%20On%20Update%20Document%20Success) (EventDispatchers|CreateEvent :!event Custom|CTUHT%20On%20Update%20Document%20Fail)))))

(event Custom|CTUHT%20On%20Update%20Document%20Success
  (params (Document%20ID :type String))
  ;[1 1 1] On Update Document
  (Development|PrintString 0 (Utilities|String|Append "Document " Document%20ID "added succesfuly") false true "(R=0.000000,G=1.000000,B=0.047720,A=1.000000)" 5.0))

(event Custom|CTUP%20On%20Load%20Document%20Fail
  (params (Document%20ID :type String))
  ;[1 1 1] On Load Document
  (Development|PrintString 0 (Utilities|String|Append "Error when loading document : " Document%20ID) false true "(R=1.000000,G=0.000000,B=0.037924,A=1.000000)" 5.0))

(event Custom|CTUP%20On%20Update%20Document%20Fail
  (params (Document%20ID :type String))
  ;[1 1 1] On Update Document
  (Development|PrintString 0 (Utilities|String|Append "Error when adding document : " Document%20ID) false true "(R=1.000000,G=0.000000,B=0.037924,A=1.000000)" 5.0))

(event Custom|CTUP%20On%20Load%20Document%20Success
  (params (Document%20ID :type String) (Document%20Snapshot :type Document%20Snapshot%20Structure))
  ;[1 1 1] On Load Document
  (bind _returnvalue (Class|FBPDataObject|FBPBeginWriteDocument))
  (bind _returnvalue_2 (Class|FBPDataObject|GetNumber (Variables|Keys|GetKey%20TimeUsedPilote) Document%20Snapshot))
  (bind _returnvalue_3 (Class|FBPDataObject|AddNumber (Variables|Keys|GetKey%20TimeUsedPilote) (+ _returnvalue_2 1.0) _returnvalue))
  (bind _player_id (Utilities|GetFireBaseSaveData)
    (:Success
      (Class|FBPFirestore|FBPUpdateDocument (Utilities|Array|MakeArray "Users" _player_id) _returnvalue_3 (EventDispatchers|CreateEvent :!event Custom|CTUP%20On%20Update%20Document%20Success) (EventDispatchers|CreateEvent :!event Custom|CTUP%20On%20Update%20Document%20Fail)))))

(event Custom|CTUP%20On%20Update%20Document%20Success
  (params (Document%20ID :type String))
  ;[1 1 1] On Update Document
  (Development|PrintString 0 (Utilities|String|Append "Document " Document%20ID "added succesfuly") false true "(R=0.000000,G=1.000000,B=0.047720,A=1.000000)" 5.0))

(event Custom|CTUPY%20On%20Load%20Document%20Fail
  (params (Document%20ID :type String))
  ;[1 1 1] On Load Document
  (Development|PrintString 0 (Utilities|String|Append "Error when loading document : " Document%20ID) false true "(R=1.000000,G=0.000000,B=0.037924,A=1.000000)" 5.0))

(event Custom|CTUPY%20On%20Update%20Document%20Fail
  (params (Document%20ID :type String))
  ;[1 1 1] On Update Document
  (Development|PrintString 0 (Utilities|String|Append "Error when adding document : " Document%20ID) false true "(R=1.000000,G=0.000000,B=0.037924,A=1.000000)" 5.0))

(event Custom|CTUPY%20On%20Load%20Document%20Success
  (params (Document%20ID :type String) (Document%20Snapshot :type Document%20Snapshot%20Structure))
  ;[1 1 1] On Load Document
  (bind _returnvalue (Class|FBPDataObject|FBPBeginWriteDocument))
  (bind _returnvalue_2 (Class|FBPDataObject|GetNumber (Variables|Keys|GetKey%20TimeUsedPyromaniac) Document%20Snapshot))
  (bind _returnvalue_3 (Class|FBPDataObject|AddNumber (Variables|Keys|GetKey%20TimeUsedPyromaniac) (+ _returnvalue_2 1.0) _returnvalue))
  (bind _player_id (Utilities|GetFireBaseSaveData)
    (:Success
      (Class|FBPFirestore|FBPUpdateDocument (Utilities|Array|MakeArray "Users" _player_id) _returnvalue_3 (EventDispatchers|CreateEvent :!event Custom|CTUPY%20On%20Update%20Document%20Success) (EventDispatchers|CreateEvent :!event Custom|CTUPY%20On%20Update%20Document%20Fail)))))

(event Custom|CTUPY%20On%20Update%20Document%20Success
  (params (Document%20ID :type String))
  ;[1 1 1] On Update Document
  (Development|PrintString 0 (Utilities|String|Append "Document " Document%20ID "added succesfuly") false true "(R=0.000000,G=1.000000,B=0.047720,A=1.000000)" 5.0))

(event Custom|CTUH%20On%20Load%20Document%20Fail
  (params (Document%20ID :type String))
  ;[1 1 1] On Load Document
  (Development|PrintString 0 (Utilities|String|Append "Error when loading document : " Document%20ID) false true "(R=1.000000,G=0.000000,B=0.037924,A=1.000000)" 5.0))

(event Custom|CTUH%20On%20Update%20Document%20Fail
  (params (Document%20ID :type String))
  ;[1 1 1] On Update Document
  (Development|PrintString 0 (Utilities|String|Append "Error when adding document : " Document%20ID) false true "(R=1.000000,G=0.000000,B=0.037924,A=1.000000)" 5.0))

(event Custom|CTUH%20On%20Load%20Document%20Success
  (params (Document%20ID :type String) (Document%20Snapshot :type Document%20Snapshot%20Structure))
  ;[1 1 1] On Load Document
  (bind _returnvalue (Class|FBPDataObject|FBPBeginWriteDocument))
  (bind _returnvalue_2 (Class|FBPDataObject|GetNumber (Variables|Keys|GetKey%20TimeUsedHealer) Document%20Snapshot))
  (bind _returnvalue_3 (Class|FBPDataObject|AddNumber (Variables|Keys|GetKey%20TimeUsedHealer) (+ _returnvalue_2 1.0) _returnvalue))
  (bind _player_id (Utilities|GetFireBaseSaveData)
    (:Success
      (Class|FBPFirestore|FBPUpdateDocument (Utilities|Array|MakeArray "Users" _player_id) _returnvalue_3 (EventDispatchers|CreateEvent :!event Custom|CTUH%20On%20Update%20Document%20Success) (EventDispatchers|CreateEvent :!event Custom|CTUH%20On%20Update%20Document%20Fail)))))

(event Custom|CTUH%20On%20Update%20Document%20Success
  (params (Document%20ID :type String))
  ;[1 1 1] On Update Document
  (Development|PrintString 0 (Utilities|String|Append "Document " Document%20ID "added succesfuly") false true "(R=0.000000,G=1.000000,B=0.047720,A=1.000000)" 5.0))

(event Custom|CTUS%20On%20Load%20Document%20Fail
  (params (Document%20ID :type String))
  ;[1 1 1] On Load Document
  (Development|PrintString 0 (Utilities|String|Append "Error when loading document : " Document%20ID) false true "(R=1.000000,G=0.000000,B=0.037924,A=1.000000)" 5.0))

(event Custom|CTUS%20On%20Update%20Document%20Fail
  (params (Document%20ID :type String))
  ;[1 1 1] On Update Document
  (Development|PrintString 0 (Utilities|String|Append "Error when adding document : " Document%20ID) false true "(R=1.000000,G=0.000000,B=0.037924,A=1.000000)" 5.0))

(event Custom|CTUS%20On%20Load%20Document%20Success
  (params (Document%20ID :type String) (Document%20Snapshot :type Document%20Snapshot%20Structure))
  ;[1 1 1] On Load Document
  (bind _returnvalue (Class|FBPDataObject|FBPBeginWriteDocument))
  (bind _returnvalue_2 (Class|FBPDataObject|GetNumber (Variables|Keys|GetKey%20TimeUsedSniper) Document%20Snapshot))
  (bind _returnvalue_3 (Class|FBPDataObject|AddNumber (Variables|Keys|GetKey%20TimeUsedSniper) (+ _returnvalue_2 1.0) _returnvalue))
  (bind _player_id (Utilities|GetFireBaseSaveData)
    (:Success
      (Class|FBPFirestore|FBPUpdateDocument (Utilities|Array|MakeArray "Users" _player_id) _returnvalue_3 (EventDispatchers|CreateEvent :!event Custom|CTUS%20On%20Update%20Document%20Success) (EventDispatchers|CreateEvent :!event Custom|CTUS%20On%20Update%20Document%20Fail)))))

(event Custom|CTUS%20On%20Update%20Document%20Success
  (params (Document%20ID :type String))
  ;[1 1 1] On Update Document
  (Development|PrintString 0 (Utilities|String|Append "Document " Document%20ID "added succesfuly") false true "(R=0.000000,G=1.000000,B=0.047720,A=1.000000)" 5.0))

(event Custom|GFCD%20On%20Load%20Document%20Fail
  (params (Document%20ID :type String))
  ;[1 1 1] On Load Document
  (Development|PrintString 0 (Utilities|String|Append "Error when loading document : " Document%20ID) false true "(R=1.000000,G=0.000000,B=0.037924,A=1.000000)" 5.0))

(event Custom|GFCD%20On%20Update%20Document%20Fail
  (params (Document%20ID :type String))
  ;[1 1 1] On Update Document
  (Development|PrintString 0 (Utilities|String|Append "Error when adding document : " Document%20ID) false true "(R=1.000000,G=0.000000,B=0.037924,A=1.000000)" 5.0))

(event Custom|GFCD%20On%20Load%20Document%20Success
  (params (Document%20ID :type String) (Document%20Snapshot :type Document%20Snapshot%20Structure))
  ;[1 1 1] On Load Document
  (bind _returnvalue (Class|FBPDataObject|FBPBeginWriteDocument))
  (bind _time_stamp (General|GetCurrentDateTime))
  (bind _returnvalue_2 (Class|FBPDataObject|AddString (Variables|Keys|GetKey%20FirstConnectionDate) _time_stamp _returnvalue))
  (bind _player_id (Utilities|GetFireBaseSaveData)
    (:Success
      (Class|FBPFirestore|FBPUpdateDocument (Utilities|Array|MakeArray "Users" _player_id) _returnvalue_2 (EventDispatchers|CreateEvent :!event Custom|GFCD%20On%20Update%20Document%20Success) (EventDispatchers|CreateEvent :!event Custom|GFCD%20On%20Update%20Document%20Fail)))))

(event Custom|GFCD%20On%20Update%20Document%20Success
  (params (Document%20ID :type String))
  ;[1 1 1] On Update Document
  (Development|PrintString 0 (Utilities|String|Append "Document " Document%20ID "added succesfuly") false true "(R=0.000000,G=1.000000,B=0.047720,A=1.000000)" 5.0))

(event Custom|GLCD%20On%20Load%20Document%20Fail
  (params (Document%20ID :type String))
  ;[1 1 1] On Load Document
  (Development|PrintString 0 (Utilities|String|Append "Error when loading document : " Document%20ID) false true "(R=1.000000,G=0.000000,B=0.037924,A=1.000000)" 5.0))

(event Custom|GLCD%20On%20Update%20Document%20Fail
  (params (Document%20ID :type String))
  ;[1 1 1] On Update Document
  (Development|PrintString 0 (Utilities|String|Append "Error when adding document : " Document%20ID) false true "(R=1.000000,G=0.000000,B=0.037924,A=1.000000)" 5.0))

(event Custom|GLCD%20On%20Load%20Document%20Success
  (params (Document%20ID :type String) (Document%20Snapshot :type Document%20Snapshot%20Structure))
  ;[1 1 1] On Load Document
  (bind _returnvalue (Class|FBPDataObject|FBPBeginWriteDocument))
  (bind _time_stamp (General|GetCurrentDateTime))
  (bind _returnvalue_2 (Class|FBPDataObject|AddString (Variables|Keys|GetKey%20LastConnectionDate) _time_stamp _returnvalue))
  (bind _player_id (Utilities|GetFireBaseSaveData)
    (:Success
      (Class|FBPFirestore|FBPUpdateDocument (Utilities|Array|MakeArray "Users" _player_id) _returnvalue_2 (EventDispatchers|CreateEvent :!event Custom|GLCD%20On%20Update%20Document%20Success) (EventDispatchers|CreateEvent :!event Custom|GLCD%20On%20Update%20Document%20Fail)))))

(event Custom|GLCD%20On%20Update%20Document%20Success
  (params (Document%20ID :type String))
  ;[1 1 1] On Update Document
  (Development|PrintString 0 (Utilities|String|Append "Document " Document%20ID "added succesfuly") false true "(R=0.000000,G=1.000000,B=0.047720,A=1.000000)" 5.0))

(event Custom|MWS%20On%20Update%20Document%20Success
  (params (DocumentId :type String))
  ;[1 1 1] On Update Document
  (Development|PrintString 0 (Utilities|String|Append "Document " DocumentId "added succesfuly") false true "(R=0.000000,G=1.000000,B=0.047720,A=1.000000)" 5.0))

(event Custom|MWS%20On%20Load%20Document%20Fail
  (params (DocumentId :type String))
  ;[1 1 1] On Load Document
  (Development|PrintString 0 (Utilities|String|Append "Error when loading document : " DocumentId) false true "(R=1.000000,G=0.000000,B=0.037924,A=1.000000)" 5.0))

(event Custom|MWS%20On%20Update%20Document%20Fail
  (params (DocumentId :type String))
  ;[1 1 1] On Update Document
  (Development|PrintString 0 (Utilities|String|Append "Error when adding document : " DocumentId) false true "(R=1.000000,G=0.000000,B=0.037924,A=1.000000)" 5.0))

(event Custom|MWS%20On%20Load%20Document%20Success
  (params (DocumentId :type String) (DocumentSnapshot :type Document%20Snapshot%20Structure))
  (bind _wavessurvivedrecordtoadd (Variables|Values|GetWavesSurvivedRecordToAdd))
  ;[1 1 1] On Load Document
  (bind _returnvalue (Class|FBPDataObject|FBPBeginWriteDocument))
  (bind _returnvalue_2 (Class|FBPDataObject|GetNumber (Variables|Keys|GetKey%20MostWavesSurvived) DocumentSnapshot))
  (if (< _returnvalue_2 _wavessurvivedrecordtoadd)
    (bind _returnvalue_3 (Class|FBPDataObject|AddNumber (Variables|Keys|GetKey%20MostWavesSurvived) _wavessurvivedrecordtoadd _returnvalue))
    (bind _player_id (Utilities|GetFireBaseSaveData)
      (:Success
        (Class|FBPFirestore|FBPUpdateDocument (Utilities|Array|MakeArray "Users" _player_id) _returnvalue_3 (EventDispatchers|CreateEvent :!event Custom|MWS%20On%20Update%20Document%20Success) (EventDispatchers|CreateEvent :!event Custom|MWS%20On%20Update%20Document%20Fail))))))

(fn AddWinsCount
  (bind _player_id (Utilities|GetFireBaseSaveData)
    (:Success
      (Class|FBPFirestore|FBPGetDocument (Utilities|Array|MakeArray "Users" _player_id) (EventDispatchers|CreateEvent :!event Custom|GWC%20On%20Load%20Document%20Success) (EventDispatchers|CreateEvent :!event Custom|GWC%20On%20Load%20Document%20Fail)))))

(fn AddLosesCount
  (bind _player_id (Utilities|GetFireBaseSaveData)
    (:Success
      (Class|FBPFirestore|FBPGetDocument (Utilities|Array|MakeArray "Users" _player_id) (EventDispatchers|CreateEvent :!event Custom|GLC%20On%20Load%20Document%20Success) (EventDispatchers|CreateEvent :!event Custom|GLC%20On%20Load%20Document%20Fail)))))

(fn UpdateTimePlayed
  (params (TimePlayedValueToAdd :type Float%20%28double-precision%29))
  (Variables|Values|SetTimePlayedValueToAdd TimePlayedValueToAdd)
  (bind _player_id (Utilities|GetFireBaseSaveData)
    (:Success
      (Class|FBPFirestore|FBPGetDocument (Utilities|Array|MakeArray "Users" _player_id) (EventDispatchers|CreateEvent :!event Custom|UTP%20On%20Load%20Document%20Success) (EventDispatchers|CreateEvent :!event Custom|UTP%20On%20Load%20Document%20Fail)))))

(fn AddTimeUsedHackerTank
  (bind _player_id (Utilities|GetFireBaseSaveData)
    (:Success
      (Class|FBPFirestore|FBPGetDocument (Utilities|Array|MakeArray "Users" _player_id) (EventDispatchers|CreateEvent :!event Custom|CTUHT%20On%20Load%20Document%20Success) (EventDispatchers|CreateEvent :!event Custom|CTUHT%20On%20Load%20Document%20Fail)))))

(fn AddTimeUsedPilote
  (bind _player_id (Utilities|GetFireBaseSaveData)
    (:Success
      (Class|FBPFirestore|FBPGetDocument (Utilities|Array|MakeArray "Users" _player_id) (EventDispatchers|CreateEvent :!event Custom|CTUP%20On%20Load%20Document%20Success) (EventDispatchers|CreateEvent :!event Custom|CTUP%20On%20Load%20Document%20Fail)))))

(fn AddTimeUsedPyromaniac
  (bind _player_id (Utilities|GetFireBaseSaveData)
    (:Success
      (Class|FBPFirestore|FBPGetDocument (Utilities|Array|MakeArray "Users" _player_id) (EventDispatchers|CreateEvent :!event Custom|CTUPY%20On%20Load%20Document%20Success) (EventDispatchers|CreateEvent :!event Custom|CTUPY%20On%20Load%20Document%20Fail)))))

(fn AddTimeUsedHealer
  (bind _player_id (Utilities|GetFireBaseSaveData)
    (:Success
      (Class|FBPFirestore|FBPGetDocument (Utilities|Array|MakeArray "Users" _player_id) (EventDispatchers|CreateEvent :!event Custom|CTUH%20On%20Load%20Document%20Success) (EventDispatchers|CreateEvent :!event Custom|CTUH%20On%20Load%20Document%20Fail)))))

(fn AddTimeUsedSniper
  (bind _player_id (Utilities|GetFireBaseSaveData)
    (:Success
      (Class|FBPFirestore|FBPGetDocument (Utilities|Array|MakeArray "Users" _player_id) (EventDispatchers|CreateEvent :!event Custom|CTUS%20On%20Load%20Document%20Success) (EventDispatchers|CreateEvent :!event Custom|CTUS%20On%20Load%20Document%20Fail)))))

(fn AddGamesPlayedCount
  (bind _player_id (Utilities|GetFireBaseSaveData)
    (:Success
      (Class|FBPFirestore|FBPGetDocument (Utilities|Array|MakeArray "Users" _player_id) (EventDispatchers|CreateEvent :!event Custom|GPC%20On%20Load%20Document%20Success) (EventDispatchers|CreateEvent :!event Custom|GPC%20On%20Load%20Document%20Fail)))))

(fn LoadFirebaseData
  (bind _returnvalue (SaveGame|DoesSaveGameExist "FirebaseData"))
  (if _returnvalue
    (bind _returnvalue_2 (SaveGame|LoadGamefromSlot "FirebaseData"))
    (bind _asbp_firebase_save (Utilities|Casting|CastToBP_FirebaseSave _returnvalue_2)
      (:then
        (return _asbp_firebase_save _returnvalue))
      (:CastFailed
        _)))
  (Development|PrintString 0 "Failed to load Firebase Data")
  (return 0 _returnvalue))

(fn InitDocuments
  (General|InitKeys)
  (bind _player_id (Utilities|GetFireBaseSaveData)
    (:Success
      (Class|FBPFirestore|FBPGetDocument (Utilities|Array|MakeArray "Users" _player_id) (EventDispatchers|CreateEvent :!event Custom|INIT%20On%20Load%20Document%20Success) (EventDispatchers|CreateEvent :!event Custom|INIT%20On%20Load%20Document%20Fail)))))

(fn InitString
  (params (Key :type String) (Default%20Value :type String) (DocumentSnapshot :type Document%20Snapshot%20Structure) (To%20Update%20Document :type Array%20of%20Data%20Object%20Value%20Structures))
  (bind _returnvalue (Class|FBPDataObject|GetString Key DocumentSnapshot))
  (if (Utilities|Enum|Equal(Enum) _returnvalue "")
    (bind _returnvalue_2 (Class|FBPDataObject|AddString Key Default%20Value To%20Update%20Document))
    (LocalVariables|SetDocument _returnvalue_2)
    (else
      (bind _returnvalue_3 (Class|FBPDataObject|AddString Key _returnvalue To%20Update%20Document))
      (LocalVariables|SetDocument _returnvalue_3)))
  (return (LocalVariables|GetDocument)))

(fn InitNumber
  (params (Key :type String) (Default%20Value :type Float%20%28double-precision%29) (DocumentSnapshot :type Document%20Snapshot%20Structure) (To%20Update%20Document :type Array%20of%20Data%20Object%20Value%20Structures))
  (bind _returnvalue (Class|FBPDataObject|GetNumber Key DocumentSnapshot))
  (if (== _returnvalue -1.0)
    (bind _returnvalue_2 (Class|FBPDataObject|AddNumber Key Default%20Value To%20Update%20Document))
    (LocalVariables|SetDocument _returnvalue_2)
    (else
      (bind _returnvalue_3 (Class|FBPDataObject|AddNumber Key _returnvalue To%20Update%20Document))
      (LocalVariables|SetDocument _returnvalue_3)))
  (return (LocalVariables|GetDocument)))

(fn InitKeys
  (Variables|Keys|SetKey%20Username "username")
  (Variables|Keys|SetKey%20GamePlayedCount "GamePlayedCount")
  (Variables|Keys|SetKey%20TimePlayed "TimePlayed")
  (Variables|Keys|SetKey%20Wins "Wins")
  (Variables|Keys|SetKey%20Loses "Loses")
  (Variables|Keys|SetKey%20TimeUsedHackerTank "TimeUsed_HackerTank")
  (Variables|Keys|SetKey%20TimeUsedPilote "TimeUsed_Pilote")
  (Variables|Keys|SetKey%20TimeUsedPyromaniac "TimeUsed_Pyromaniac")
  (Variables|Keys|SetKey%20TimeUsedHealer "TimeUsed_Healer")
  (Variables|Keys|SetKey%20TimeUsedSniper "TimeUsed_Sniper")
  (Variables|Keys|SetKey%20FirstConnectionDate "FirstConnectionDate")
  (Variables|Keys|SetKey%20LastConnectionDate "LastConnectionDate")
  (Variables|Keys|SetKey%20MostWavesSurvived "MostWavesSurvived"))

(fn GetAllDocument
  (params (DocumentSnapshot :type Document%20Snapshot%20Structure) (To%20Update%20Document :type Array%20of%20Data%20Object%20Value%20Structures))
  (bind _updated_document (General|InitString (Variables|Keys|GetKey%20FirstConnectionDate) "0000-00-00T00:00:00Z" DocumentSnapshot To%20Update%20Document))
  (bind _updated_document_2 (General|InitString (Variables|Keys|GetKey%20LastConnectionDate) "0000-00-00T00:00:00Z" DocumentSnapshot _updated_document))
  (bind _updated_document_3 (General|InitString (Variables|Keys|GetKey%20Username) "Default_Username" DocumentSnapshot _updated_document_2))
  (bind _updated_document_4 (General|InitNumber (Variables|Keys|GetKey%20GamePlayedCount) 0.0 DocumentSnapshot _updated_document_3))
  (bind _updated_document_5 (General|InitNumber (Variables|Keys|GetKey%20Wins) 0.0 DocumentSnapshot _updated_document_4))
  (bind _updated_document_6 (General|InitNumber (Variables|Keys|GetKey%20Loses) 0.0 DocumentSnapshot _updated_document_5))
  (bind _updated_document_7 (General|InitNumber (Variables|Keys|GetKey%20TimePlayed) 0.0 DocumentSnapshot _updated_document_6))
  (bind _updated_document_8 (General|InitNumber (Variables|Keys|GetKey%20TimeUsedHackerTank) 0.0 DocumentSnapshot _updated_document_7))
  (bind _updated_document_9 (General|InitNumber (Variables|Keys|GetKey%20TimeUsedPilote) 0.0 DocumentSnapshot _updated_document_8))
  (bind _updated_document_10 (General|InitNumber (Variables|Keys|GetKey%20TimeUsedPyromaniac) 0.0 DocumentSnapshot _updated_document_9))
  (bind _updated_document_11 (General|InitNumber (Variables|Keys|GetKey%20TimeUsedHealer) 0.0 DocumentSnapshot _updated_document_10))
  (bind _updated_document_12 (General|InitNumber (Variables|Keys|GetKey%20TimeUsedSniper) 0.0 DocumentSnapshot _updated_document_11))
  (bind _updated_document_13 (General|InitNumber (Variables|Keys|GetKey%20MostWavesSurvived) 0.0 DocumentSnapshot _updated_document_12))
  (return _updated_document_13))

(fn GetCurrentDateTime
  (bind _returnvalue (Math|DateTime|Now))
  (bind (_year _month _day _hour _minute _second) (Math|DateTime|BreakDateTime _returnvalue))
  (return (Utilities|String|Append (Utilities|String|ToString(Integer) _year) "-" (Utilities|String|ToString(Integer) _month) "-" (Utilities|String|ToString(Integer) _day) "T" (Utilities|String|ToString(Integer) _hour) ":" (Utilities|String|ToString(Integer) _minute) ":" (Utilities|String|ToString(Integer) _second) "Z")))

(fn AddFirstConnetionDate
  (bind _player_id (Utilities|GetFireBaseSaveData)
    (:Success
      (Class|FBPFirestore|FBPGetDocument (Utilities|Array|MakeArray "Users" _player_id) (EventDispatchers|CreateEvent :!event Custom|GFCD%20On%20Load%20Document%20Success) (EventDispatchers|CreateEvent :!event Custom|GFCD%20On%20Load%20Document%20Fail)))))

(fn UpdateLastConnectionDate
  (bind _player_id (Utilities|GetFireBaseSaveData)
    (:Success
      (Class|FBPFirestore|FBPGetDocument (Utilities|Array|MakeArray "Users" _player_id) (EventDispatchers|CreateEvent :!event Custom|GLCD%20On%20Load%20Document%20Success) (EventDispatchers|CreateEvent :!event Custom|GLCD%20On%20Load%20Document%20Fail)))))

(fn UpdateWavesSurvivedRecord
  (params (WavesSurvivedRecordToAdd :type Float%20%28double-precision%29))
  (Variables|Values|SetWavesSurvivedRecordToAdd WavesSurvivedRecordToAdd)
  (bind _player_id (Utilities|GetFireBaseSaveData)
    (:Success
      (Class|FBPFirestore|FBPGetDocument (Utilities|Array|MakeArray "Users" _player_id) (EventDispatchers|CreateEvent :!event Custom|MWS%20On%20Load%20Document%20Success) (EventDispatchers|CreateEvent :!event Custom|MWS%20On%20Load%20Document%20Fail)))))