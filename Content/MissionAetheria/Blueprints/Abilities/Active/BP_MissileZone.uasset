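; Active ability that fires a timed volley of pooled missiles from the actor's position, each randomly offset in Y and Z.
; Use starts a delayed loop that sets IsVFXVisible and has the owning player server-spawn each missile from the missile pool, then reloads the ability on completion.
; UseDuration derives from missile count and spacing, and SetVFXVisibility spawns an auto-released muzzle effect at its own random offset.
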(event Custom|OnAbilitieUsed
  (bind _returnvalue (Transformation|GetActorTransform))
  (Utilities|ForLoopwithDelay 1 (Variables|Default|GetnumberMissiles) (Variables|Default|GettimeBewteenMissiles)
    (:LoopBody
      (Variables|Default|SetIsVFXVisible true)
      (bind _playerowner (Variables|Default|GetPlayerOwner)
        (:then
          (Default|ServerSpawnfromPool _playerowner (Variables|Default|GetAC_MissilePool) (Math|Transform|MakeTransform (Math|Vector|MakeVector (.x (.location _returnvalue)) (Math|Random|RandomFloatinRange (- (.y (.location _returnvalue)) 1e+02) (+ (.y (.location _returnvalue)) 1e+02)) (Math|Random|RandomFloatinRange (- (.z (.location _returnvalue)) 1e+02) (+ (.z (.location _returnvalue)) 1e+02))) (.rotation _returnvalue) (.scale _returnvalue))))
        (:else)))
    (:Completed
      (CallFunction|PlayerReloadAbility)
      (CallFunction|OnReload)
      (Development|PrintString "All Missile launched !"))))

(event EventBeginPlay
  (Variables|Default|SetUseDuration (* (Variables|Default|GettimeBewteenMissiles) (Variables|Default|GetnumberMissiles))))

(fn ConstructionScript
  (|CallParentFunction))

(fn RandomTransform
  (params (transform :type Transform)))

(fn Use
  (|CallParentFunction)
  (CallFunction|OnAbilitieUsed))

(fn TrytoUse
  (CallFunction|PlayerUseAbility)
  (|CallParentFunction))

(fn SetVFXVisibility
  (params (ShouldbeVisible :type Boolean))
  (bind _returnvalue (Transformation|GetActorTransform))
  (if ShouldbeVisible
    (Niagara|SpawnSystematLocation "/Game/MissionAetheria/VFX/Niagara/NS_MuzzleShot_Missile.NS_MuzzleShot_Missile" (Math|Vector|MakeVector (.x (.location _returnvalue)) (Math|Random|RandomFloatinRange (- (.y (.location _returnvalue)) 1e+02) (+ (.y (.location _returnvalue)) 1e+02)) (Math|Random|RandomFloatinRange (- (.z (.location _returnvalue)) 1e+02) (+ (.z (.location _returnvalue)) 1e+02))) (.rotation _returnvalue) (.scale _returnvalue) true true "AutoRelease")))