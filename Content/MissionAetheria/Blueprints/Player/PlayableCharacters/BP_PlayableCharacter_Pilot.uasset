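; Playable Pilot character, a flying ship with minigun weapons and a missile zone ability, built on a shared character parent.
; The active ability toggles between two cameras and updates the HUD, switching Shoot between firing weapons and using the missile zone with camera shake.
; Movement follows control rotation with vertical input and drives Niagara thruster effects, while being downed switches Flying to Falling.
; It also maintains a second cannister set and resizes its capsule based on character attraction.
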(event Input|EnhancedActionEvents|EnhancedInputActionIA_Shoot
  (params (ActionValue :type Boolean) (ElapsedSeconds :type Float%20%28double-precision%29) (TriggeredSeconds :type Float%20%28double-precision%29) (InputAction :type Input%20Action%20Object%20Reference :default "/Game/MissionAetheria/Inputs/Actions/IA_Shoot.IA_Shoot"))
  ;[1 1 1] Shoot
  (:Triggered
    (if (not (CallFunction|Can'tMove))
      (if (not (Variables|Default|GetCameraAbility))
        (for _array_element (Variables|Default|GetWeapon)
          (Default|TrytoFire _array_element)))))
  (:Started
    (if (not (CallFunction|Can'tMove))
      (if (Variables|Default|GetCameraAbility)
        (if (Variables|/Game/MissionAetheria/Blueprints/Abilities/Active/BP_BaseActiveAbility.BP_BaseActiveAbility_C|GetIsReadyToBeUsed (CallFunction|GetMissileZone))
          (Default|TrytoUse (CallFunction|GetMissileZone))
          (CameraShake|Start (Variables|Default|GetCameraShakeSource_0)))))))

(event Input|EnhancedActionEvents|EnhancedInputActionIA_Look
  (params (ActionValue :type Vector%202D%20Structure) (ElapsedSeconds :type Float%20%28double-precision%29) (TriggeredSeconds :type Float%20%28double-precision%29) (InputAction :type Input%20Action%20Object%20Reference :default "/Game/ThirdPerson/Input/Actions/IA_Look.IA_Look"))
  (if (not (Variables|Default|GetIsDown))
    (Transformation|SetWorldRotation (Variables|Default|GetBP_Minigun) (Transformation|GetWorldRotation (Variables|Default|GetTarget)) false false)))

(event Input|EnhancedActionEvents|EnhancedInputActionIA_UseActiveAbility
  (params (ActionValue :type Boolean) (ElapsedSeconds :type Float%20%28double-precision%29) (TriggeredSeconds :type Float%20%28double-precision%29) (InputAction :type Input%20Action%20Object%20Reference :default "/Game/MissionAetheria/Inputs/Actions/IA_UseActiveAbility.IA_UseActiveAbility"))
  (:Started
    (CallFunction|SwitchCamera)))

(event Input|EnhancedActionEvents|EnhancedInputActionIA_FlyUpDown
  (params (ActionValue :type Vector%202D%20Structure) (ElapsedSeconds :type Float%20%28double-precision%29) (TriggeredSeconds :type Float%20%28double-precision%29) (InputAction :type Input%20Action%20Object%20Reference :default "/Game/MissionAetheria/Inputs/Actions/IA_FlyUpDown.IA_FlyUpDown"))
  (if (not (CallFunction|Can'tMove))
    (Pawn|Input|AddMovementInput (Transformation|GetActorUpVector (Pawn|GetController)) (.x ActionValue) false)))

(event Input|EnhancedActionEvents|EnhancedInputActionIA_Move
  (params (ActionValue :type Vector%202D%20Structure) (ElapsedSeconds :type Float%20%28double-precision%29) (TriggeredSeconds :type Float%20%28double-precision%29) (InputAction :type Input%20Action%20Object%20Reference :default "/Game/ThirdPerson/Input/Actions/IA_Move.IA_Move"))
  (:Triggered
    (if (not (CallFunction|Can'tMove))
      (CallFunction|Move 0.0 0.0)))
  (:Canceled
    (CallFunction|ChangeThrustersVFXParams 5.0 0.5 :!label _label))
  (:Completed
    (goto _label)))

(event EventBeginPlay
  (CallFunction|ChangeThrustersVFXParams 5.0 0.0)
  (CallFunction|SetData "NewEnumerator0")
  (Variables|Default|SetWeaponsAbilitiesParent (Variables|Default|GetSM_PilotShip))
  (|CallParentFunction)
  (Collision|IgnoreActorwhenMoving (Variables|Default|GetSM_PilotShip) (Variables|Default|GetMinigunRef) true)
  (for _array_element (Utilities|Array|MakeArray (Variables|Default|GetCan_0) (Variables|Default|GetCan_1) (Variables|Default|GetCan_2))
    (CallFunction|AddCannistertotheArray _array_element))
  (Utilities|Array|Clear (Variables|Default|GetSecondCannister))
  (for _array_element_2 (Utilities|Array|MakeArray (Variables|Default|GetCan_3) (Variables|Default|GetCan_4) (Variables|Default|GetCan_5))
    (bind _asbp_cannister (Utilities|Casting|CastToBP_Cannister (Variables|/Script/Engine.ChildActorComponent|GetChildActor _array_element_2)))
    (Utilities|Array|AddUnique (Variables|Default|GetSecondCannister) _asbp_cannister)))

(fn ConstructionScript
  (|CallParentFunction))

(fn SwitchCamera
  (bind _camera (Variables|Default|GetCamera))
  (bind _cameraweapon (Variables|Default|GetCameraWeapon))
  (bind _returnvalue (Components|Activation|IsActive _cameraweapon))
  (bind _returnvalue_2 (not _returnvalue))
  (Components|Activation|SetActive _camera (not (Components|Activation|IsActive _camera)) false)
  (Variables|Default|SetCameraAbility _returnvalue_2)
  (Components|Activation|SetActive _cameraweapon _returnvalue_2 false)
  (Default|ChangePiloteMuni (Variables|/Game/MissionAetheria/Blueprints/PlayerControllers/PC_BasePlayerController.PC_BasePlayerController_C|GetWBPStageGeneral (CallFunction|GetPlayerController)) (Components|Activation|IsActive (Variables|Default|GetCamera))))

(fn GetMissileZone
  (Variables|Default|GetMissileZoneRef
    (:then
      (return (Variables|Default|GetMissileZoneRef)))
    (:else
      (bind _asbp_missile_zone (Utilities|Casting|CastToBP_MissileZone (Variables|/Script/Engine.ChildActorComponent|GetChildActor (Variables|Default|GetBP_MissileZone)))
        (:then
          (Variables|Default|SetMissileZoneRef _asbp_missile_zone)
          (return (Variables|Default|GetMissileZoneRef)))
        (:CastFailed
          (Development|PrintString "BP_PlayableCharacter_Pilot | Cast to BP_MissileZone failed !" true true "(R=1.000000,G=0.000000,B=0.000000,A=1.000000)"))))))

(fn UpdateCannisters
  (|CallParentFunction)
  (CallFunction|UpdateCannisterArray (Variables|Default|GetSecondCannister)))

(fn ChangeThrustersVFXParams
  (params (newRate :type Float%20%28double-precision%29) (newSize :type Float%20%28double-precision%29))
  (if (not (== newRate (Variables|Default|GetcurrentThrustersRate)))
    (bind _output_get (Variables|Default|SetcurrentThrustersRate newRate))
    (Niagara|SetNiagaraVariable(Float) (Variables|Default|GetNS_Pilot_Thrusters) "SpawnRate" _output_get)
    (Niagara|SetNiagaraVariable(Float) (Variables|Default|GetNS_Pilot_Thrusters1) "SpawnRate" (Variables|Default|GetcurrentThrustersRate))
    (Niagara|SetNiagaraVariable(Float) (Variables|Default|GetNS_Pilot_Thrusters) "MeshMaxSize" newSize)
    (Niagara|SetNiagaraVariable(Float) (Variables|Default|GetNS_Pilot_Thrusters1) "MeshMaxSize" newSize)))

(fn SetIsDown
  (params (IsDown :type Boolean))
  (bind _charactermovement (Variables|Character|GetCharacterMovement))
  (if IsDown
    (Pawn|Components|CharacterMovement|SetMovementMode _charactermovement "MOVE_Falling" 0)
    (else
      (Pawn|Components|CharacterMovement|SetMovementMode _charactermovement "MOVE_Flying" 0)))
  (|CallParentFunction IsDown))

(fn Move
  (params (x :type Float%20%28double-precision%29) (y :type Float%20%28double-precision%29))
  (bind _returnvalue (Pawn|GetControlRotation :!class /Script/Engine.Pawn))
  (CallFunction|ChangeThrustersVFXParams 25.0 1.5)
  (Pawn|Input|AddMovementInput (Math|Vector|GetRightVector (Pawn|GetControlRotation :!class /Script/Engine.Pawn)) x false)
  (Pawn|Input|AddMovementInput (Math|Vector|GetForwardVector (Math|Rotator|MakeRotator (.roll _returnvalue) 0.0 (.yaw _returnvalue))) y false))

(fn UpdatePilotCollisionSize
  (bind _capsulecomponent (Variables|Default|GetCapsuleComponent))
  (if (Variables|Default|GetCanAttractCharacter)
    (Components|Capsule|SetCapsuleHalfHeight _capsulecomponent 1.9e+02 true)
    (else
      (Components|Capsule|SetCapsuleHalfHeight _capsulecomponent 2.8e+02 true))))