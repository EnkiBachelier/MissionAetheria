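; Game mode for the role choice stage, which spawns players and manages the loading screen on entry.
; PostLogin spawns a BP_Player_RoleChoice at a player start and has the joining PC_RoleChoice possess it.
; BeginPlay shows the GI_MissionAetheria loading screen, resuming any existing animation time, and starts a short timer, presumably for DisableLoadingScreen to hide it.
; A helper lazily caches the cast game instance.
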(event EventBeginPlay
  (bind _gameinstance (CallFunction|GetGameInstance))
  (bind _loadingscreen (Variables|/Game/MissionAetheria/Blueprints/GameInstance/GI_MissionAetheria.GI_MissionAetheria_C|GetLoadingScreen _gameinstance))
  (Utilities|IsValid _loadingscreen
    (:Is%20Valid
      (bind _time (Default|GetCurrentAnimationTime _loadingscreen))
      (Default|SetLoadingScreenVisibility _gameinstance true _time))
    (:Is%20Not%20Valid
      (Default|SetLoadingScreenVisibility _gameinstance true 0.0)))
  (Utilities|Time|SetTimerbyEvent (EventDispatchers|CreateEvent :!event DisableLoadingScreen) 0.5))

(event EventPostLogin
  (params (NewPlayer :type Player%20Controller%20Object%20Reference))
  (bind _aspc_role_choice (Utilities|Casting|CastToPC_RoleChoice NewPlayer))
  (bind _returnvalue (Game|SpawnActorfromClass "/Game/MissionAetheria/Blueprints/Player/BP_Player_RoleChoice.BP_Player_RoleChoice_C" (Transformation|GetActorTransform (Class|GameModeBase|FindPlayerStart)) "Undefined" "MultiplyWithRoot" 0 0))
  (Pawn|Possess _aspc_role_choice _returnvalue))

(fn ConstructionScript)

(fn GetGameInstance
  (Utilities|IsValid (Variables|Default|GetGameInstance)
    (:Is%20Valid
      (return (Variables|Default|GetGameInstance)))
    (:Is%20Not%20Valid
      (bind _asgi_mission_aetheria (Utilities|Casting|CastToGI_MissionAetheria (Game|GetGameInstance))
        (:then
          (Variables|Default|SetGameInstance _asgi_mission_aetheria)
          (return (Variables|Default|GetGameInstance)))
        (:CastFailed
          (Development|PrintString "GM_RoleChoice | Couldn't cast the GameInstance to GI_MissionAetheria" true true "(R=0.000000,G=0.660000,B=1.000000,A=1.000000)" 1e+01))))))

(fn DisableLoadingScreen
  (Default|SetLoadingScreenVisibility (CallFunction|GetGameInstance) false 0.0))