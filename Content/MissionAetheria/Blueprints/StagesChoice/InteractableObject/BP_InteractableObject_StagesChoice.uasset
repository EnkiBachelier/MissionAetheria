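; Base interactable object for the stage-choice scene, detecting the stage-choice player through a sphere overlap.
; Overlap begin and end call empty BeginOverlap and EndOverlap hooks, with a shared timed lock that ignores further overlaps briefly.
; Empty FirstInteraction and SecondInteraction functions are also declared.
; When IsPlaced is set, the construction script traces toward and past the world origin, aligning the actor's up axis to the impact normal.
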(event OnComponentBeginOverlap(Sphere)
  (params (OverlappedComponent :type Primitive%20Component%20Object%20Reference) (OtherActor :type Actor%20Object%20Reference) (OtherComp :type Primitive%20Component%20Object%20Reference) (OtherBodyIndex :type Integer) (bFromSweep :type Boolean) (SweepResult :type Hit%20Result%20Structure%20%28by%20ref%29))
  (if (not (Variables|Default|GetIsOverlappingDetectionStop))
    (if (== (Utilities|GetClass OtherActor) "/Game/MissionAetheria/Blueprints/Player/BP_Player_StagesChoice.BP_Player_StagesChoice_C")
      (bind _asbp_player_stages_choice (Utilities|Casting|CastToBP_Player_StagesChoice OtherActor))
      (CallFunction|BeginOverlap _asbp_player_stages_choice)
      (Variables|Default|SetIsOverlappingDetectionStop true)
      (Utilities|FlowControl|Delay (Variables|Default|GetDuration))
      (Variables|Default|SetIsOverlappingDetectionStop false))))

(event OnComponentEndOverlap(Sphere)
  (params (OverlappedComponent :type Primitive%20Component%20Object%20Reference) (OtherActor :type Actor%20Object%20Reference) (OtherComp :type Primitive%20Component%20Object%20Reference) (OtherBodyIndex :type Integer))
  (if (not (Variables|Default|GetIsOverlappingDetectionStop))
    (if (== (Utilities|GetClass OtherActor) "/Game/MissionAetheria/Blueprints/Player/BP_Player_StagesChoice.BP_Player_StagesChoice_C")
      (bind _asbp_player_stages_choice (Utilities|Casting|CastToBP_Player_StagesChoice OtherActor))
      (CallFunction|EndOverlap _asbp_player_stages_choice)
      (Variables|Default|SetIsOverlappingDetectionStop true)
      (Utilities|FlowControl|Delay (Variables|Default|GetDuration))
      (Variables|Default|SetIsOverlappingDetectionStop false))))

(event EventBeginPlay)

(event EventTick
  (params (DeltaSeconds :type Float%20%28single-precision%29)))

(fn ConstructionScript
  (bind _staticmesh (Variables|Default|GetStaticMesh))
  (bind _returnvalue (Transformation|GetWorldLocation _staticmesh))
  (if (Variables|Default|GetIsPlaced)
    (bind _outhit (Collision|LineTraceByChannel _returnvalue (* _returnvalue -1e+02) "TraceTypeQuery1" false 0 "ForDuration"))
    (Transformation|SetActorRotation (Math|Rotator|MakeRotfromZ (.impactnormal _outhit)))))

(fn FirstInteraction
  (params (player :type BP%20Player%20Stages%20Choice%20Object%20Reference)))

(fn BeginOverlap
  (params (Player :type BP%20Player%20Stages%20Choice%20Object%20Reference)))

(fn EndOverlap
  (params (Player :type BP%20Player%20Stages%20Choice%20Object%20Reference)))

(fn SecondInteraction
  (params (Player :type BP%20Player%20Stages%20Choice%20Object%20Reference)))