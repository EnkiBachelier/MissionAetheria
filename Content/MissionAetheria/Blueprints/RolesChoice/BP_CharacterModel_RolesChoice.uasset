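; Preview character actor for the role selection screen, configured by its CharacterRole.
; The construction script tags it with the role name, loads the role's mesh from the characters data table and points its scene capture at that role's render target.
; SetChoose forwards the confirmation state to the AB_Template_RoleChoice anim instance, which is cast and cached on first use.
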(event Custom|SetChoose
  (params (isConfirmed :type Boolean))
  (Default|SetChoose (CallFunction|GetAnimBlueprint) isConfirmed))

(event EventBeginPlay)

(event Collision|EventActorBeginOverlap
  (params (OtherActor :type Actor%20Object%20Reference)))

(event EventTick
  (params (DeltaSeconds :type Float%20%28single-precision%29)))

(fn ConstructionScript
  (bind _characterrole (Variables|Default|GetCharacterRole))
  (bind _role_targettextures (Variables|Default|GetRole_TargetTextures))
  (bind _characterrole_2 (Variables|Default|GetCharacterRole))
  (bind (_value _returnvalue) (Utilities|Map|Find _role_targettextures _characterrole_2))
  (bind _returnvalue_2 (Utilities|String|EnumtoString _characterrole))
  (bind _returnvalue_3 (Utilities|String|StringToName _returnvalue_2))
  (Variables|Default|SetTags (Utilities|Array|MakeArray _returnvalue_3))
  (Utilities|FlowControl|Sequence
    (:then_0
      (bind _returnvalue_4 (Utilities|GetDataTableRow "/Game/MissionAetheria/Datatables/DataTable_Characters.DataTable_Characters" _returnvalue_3)
        (:then
          (Variables|/Script/Engine.SkeletalMeshComponent|SetSkeletalMeshAsset (Variables|Default|GetSkeletalMesh) (.mesh _returnvalue_4))
          (Utilities|FlowControl|Sequence))))
    (:then_1
      (if _returnvalue
        (Variables|/Script/Engine.SceneCaptureComponent2D|SetTextureTarget (Variables|Default|GetSceneCaptureComponent2D) _value)))))

(fn GetAnimBlueprint
  (Variables|Default|GetAnimBlueprint
    (:then
      _)
    (:else
      (bind _asab_template_role_choice (Utilities|Casting|CastToAB_Template_RoleChoice (Components|SkeletalMesh|GetAnimInstance (Variables|Default|GetSkeletalMesh))))
      (Variables|Default|SetAnimBlueprint _asab_template_role_choice)))
  (return (Variables|Default|GetAnimBlueprint)))