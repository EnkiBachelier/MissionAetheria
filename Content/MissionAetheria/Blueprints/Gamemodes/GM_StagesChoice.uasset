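; Game mode for the stage selection level, handling player spawning, loading screen visibility and the switch to a chosen stage.
; BeginPlay shows the loading screen, binds every BP_Slot's start-level event, caches PlayerStarts and starts a timer.
; SpawnPlayer replaces each controller's pawn with a character at the next PlayerStart.
; On authority, LoadLevelFromDatatable saves the slot's DataTable row to the GameInstance and requests a server level switch.
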(event EventBeginPlay
  (bind _gameinstance (CallFunction|GetGameInstance))
  (bind _loadingscreen (Variables|/Game/MissionAetheria/Blueprints/GameInstance/GI_MissionAetheria.GI_MissionAetheria_C|GetLoadingScreen _gameinstance))
  (Utilities|IsValid _loadingscreen
    (:Is%20Valid
      (bind _time (Default|GetCurrentAnimationTime _loadingscreen))
      (Default|SetLoadingScreenVisibility _gameinstance true _time))
    (:Is%20Not%20Valid
      (Default|SetLoadingScreenVisibility _gameinstance true 0.0)))
  (bind _outactors (Actor|GetAllActorsOfClass "/Game/MissionAetheria/Blueprints/StagesChoice/InteractableObject/Slots/BP_Slot.BP_Slot_C"))
  (for _array_element _outactors
    (EventDispatchers|BindEventtoOnStartLevel _array_element (EventDispatchers|CreateEvent :!event LoadLevelfromDatatable))
    (bind _outactors_2 (Actor|GetAllActorsOfClass "/Script/Engine.PlayerStart"))
    (Variables|Default|SetallPlayerStarts _outactors_2)
    (Utilities|Time|SetTimerbyEvent (EventDispatchers|CreateEvent :!event DisableLoadingScreen) 1.0)))

(event EventPostLogin
  (params (NewPlayer :type Player%20Controller%20Object%20Reference))
  (bind _returnvalue (Utilities|Array|Add (Variables|Default|GetAll_Pc's) NewPlayer))
  (Variables|/Game/MissionAetheria/Blueprints/GameInstance/GI_MissionAetheria.GI_MissionAetheria_C|SetCurrentNumberOfPlayers (CallFunction|GetGameInstance) (+ _returnvalue 1)))

(event EventOnSwapPlayerControllers
  (params (OldPC :type Player%20Controller%20Object%20Reference) (NewPC :type Player%20Controller%20Object%20Reference))
  (Utilities|Array|Add (Variables|Default|GetAll_Pc's) NewPC))

(event EventOnLogout
  (params (ExitingController :type Controller%20Object%20Reference))
  (bind _aspc_stages_choice (Utilities|Casting|CastToPC_StagesChoice ExitingController))
  (Utilities|Array|RemoveItem (Variables|Default|GetAll_Pc's) _aspc_stages_choice))

(fn ConstructionScript)

(fn SetGeneralStagesChoiceUI
  (params (newUI :type WBP%20General%20Stages%20Choice%20Object%20Reference))
  (bind _output_get (Variables|Default|SetGeneralStagesChoiceUI newUI))
  (EventDispatchers|BindEventtoOnStartLevelButtonClicked _output_get (EventDispatchers|CreateEvent :!event LoadLevelfromDatatable)))

(fn LoadLevelfromDatatable
  (params (Slot :type BP%20Slot%20Object%20Reference))
  (bind _datatablerowtoload (Variables|/Game/MissionAetheria/Blueprints/StagesChoice/InteractableObject/Slots/BP_Slot.BP_Slot_C|GetDataTableRowToLoad Slot))
  (bind _asbp_player_stages_choice (Utilities|Casting|CastToBP_Player_StagesChoice (Game|GetPlayerCharacter 0)))
  (Default|ServerActiveSlotPanel _asbp_player_stages_choice false Slot false)
  (Networking|SwitchHasAuthority
    (:Authority
      (bind _returnvalue (Utilities|GetDataTableRow "/Game/MissionAetheria/Datatables/DataTable_Stages.DataTable_Stages" _datatablerowtoload)
        (:then
          (Default|SaveDatatableRow (Variables|Default|GetGameInstance) _datatablerowtoload)
          (Default|ServerSwitchLevel (CallFunction|GetPlayerController) (Utilities|String|ToString(Name) (.LevelToLoad (Utilities|Struct|BreakStruct_LevelData _returnvalue)))))))))

(fn FindRandomPlayerStart
  (bind _outactors (Actor|GetAllActorsOfClass "/Script/Engine.PlayerStart"))
  (return (Transformation|GetActorTransform (Utilities|Array|Get(acopy) _outactors (Math|Random|RandomIntegerinRange 0 (- (Utilities|Array|Length _outactors) 1))))))

(fn SpawnPlayer
  (params (PlayerController :type Player%20Controller%20Object%20Reference) (player :type Struct%20Player%20Structure))
  (bind _returnvalue (Pawn|GetControlledPawn PlayerController))
  (bind _output_get (Variables|Default|SetPlayer player))
  (Utilities|IsValid _returnvalue
    (:Is%20Valid
      (Actor|DestroyActor _returnvalue))
    (:Is%20Not%20Valid
      _))
  (bind _returnvalue_2 (Game|SpawnActorfromClass "/Game/MissionAetheria/Blueprints/Player/BP_Player_StagesChoice.BP_Player_StagesChoice_C" (Transformation|GetActorTransform (Utilities|Array|Get(acopy) (Variables|Default|GetallPlayerStarts) (Variables|Default|GetcurrentPlayerCount))) "AdjustIfPossibleButAlwaysSpawn" "MultiplyWithRoot" 0 player 0))
  (Pawn|Possess PlayerController _returnvalue_2)
  (Utilities|Array|Add (Variables|/Game/MissionAetheria/Blueprints/GameInstance/GI_MissionAetheria.GI_MissionAetheria_C|GetCharactersInStageChoice (Variables|Default|GetGameInstance)) _returnvalue_2)
  (Math|Integer|IncrementInt (Variables|Default|GetcurrentPlayerCount)))

(fn GetGameInstance
  (Utilities|IsValid (Variables|Default|GetGameInstance)
    (:Is%20Valid
      (return (Variables|Default|GetGameInstance)))
    (:Is%20Not%20Valid
      (bind _asgi_mission_aetheria (Utilities|Casting|CastToGI_MissionAetheria (Game|GetGameInstance))
        (:then
          (Variables|Default|SetGameInstance _asgi_mission_aetheria)
          (return (Variables|Default|GetGameInstance)))
        (:CastFailed
          (Development|PrintString "GM_StagesChoices/BeginPlay | Couldn't cast the GameInstance to GI_MissionAetheria" true true "(R=0.000000,G=0.660000,B=1.000000,A=1.000000)" 1e+01))))))

(fn GetPlayerController
  (Utilities|IsValid (Variables|Default|GetplayerController)
    (:Is%20Valid
      _)
    (:Is%20Not%20Valid
      (bind _aspc_stages_choice (Utilities|Casting|CastToPC_StagesChoice (Game|GetPlayerController 0)))
      (Variables|Default|SetplayerController _aspc_stages_choice)))
  (return (Variables|Default|GetplayerController)))

(fn GetGameState
  (Variables|Default|GetGS_BaseStage
    (:then
      _)
    (:else
      (bind _asgs_base_stage (Utilities|Casting|CastToGS_BaseStage (Game|GetGameState)))
      (Variables|Default|SetGS_BaseStage _asgs_base_stage)))
  (return (Variables|Default|GetGS_BaseStage)))

(fn DisableLoadingScreen
  (Default|SetLoadingScreenVisibility (CallFunction|GetGameInstance) false 0.0))