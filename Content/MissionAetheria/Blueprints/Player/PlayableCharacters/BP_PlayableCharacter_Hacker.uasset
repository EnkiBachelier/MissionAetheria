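; BP_PlayableCharacter_Hacker is the Hacker variant of a playable character, built on a parent character Blueprint.
; On BeginPlay it sets its character data to a fixed enum entry, then runs the parent's BeginPlay.
; Its Init runs the parent's Init and then registers three canisters, Can0 to Can2, in the canister array.
; The construction script only calls the parent's.
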(event EventBeginPlay
  (CallFunction|SetData "NewEnumerator3")
  (|CallParentFunction))

(fn ConstructionScript
  (|CallParentFunction))

(fn Init
  (|CallParentFunction)
  (for _array_element (Utilities|Array|MakeArray (Variables|Default|GetCan_0) (Variables|Default|GetCan_1) (Variables|Default|GetCan_2))
    (CallFunction|AddCannistertotheArray _array_element)))