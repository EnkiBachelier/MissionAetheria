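; BP_SniperGrenade is a throwable grenade that explodes as soon as its collision overlaps an actor whose class is not in an ignore list.
; The overlap plays a Wwise sound, disables collision, fires a radial impulse and applies radial damage.
; It also spawns a Niagara explosion, starts a camera shake and hides the mesh.
; After a short delay, it destroys the effect and itself.
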(event OnComponentBeginOverlap(Collision)
  (params (OverlappedComponent :type Primitive%20Component%20Object%20Reference) (OtherActor :type Actor%20Object%20Reference) (OtherComp :type Primitive%20Component%20Object%20Reference) (OtherBodyIndex :type Integer) (bFromSweep :type Boolean) (SweepResult :type Hit%20Result%20Structure%20%28by%20ref%29))
  (bind _returnvalue (Transformation|GetActorLocation))
  ;[1 1 1 0.505] On collision set velocity to 0, stick the grenade where she landed and explode after X seconds
  (if (not (Utilities|Array|ContainsItem (Variables|Default|GetActorToIgnore) (Utilities|GetClass OtherActor)))
    (Class|AkGameplayStatics|PostEventatLocation "/Game/WwiseAudio/Events/Default_Work_Unit/SFX_Character/Abilitys/Sniper/Play_Grenade_Impule.Play_Grenade_Impule" (Transformation|GetWorldLocation (Variables|Default|GetSK_SniperGrenade)) "0, 0, 0")
    (Collision|SetCollisionResponsetoAllChannels (Variables|Default|GetCollision) "ECR_Ignore")
    (Transformation|SetWorldLocation (Variables|Default|GetSK_SniperGrenade) (Transformation|GetWorldLocation (Variables|Default|GetSK_SniperGrenade)) false false)
    (Class|RadialForceComponent|FireImpulse (Variables|Default|GetRadialForce))
    (Game|Damage|ApplyRadialDamage (Variables|Default|GetAmount%20Damage) _returnvalue 4e+02 "/Script/Engine.DamageType" 0 0 0 false "ECC_Visibility")
    (bind _returnvalue_2 (Niagara|SpawnSystematLocation "/Game/MissionAetheria/VFX/Niagara/NS_StylizedExplosion.NS_StylizedExplosion" _returnvalue))
    (CameraShake|Start (Variables|Default|GetCameraShakeGrenade))
    (Rendering|SetVisibility (Variables|Default|GetSK_SniperGrenade) false false)
    (Utilities|FlowControl|Delay 1.5)
    (Components|DestroyComponent _returnvalue_2)
    (Actor|DestroyActor)))

(fn ConstructionScript)