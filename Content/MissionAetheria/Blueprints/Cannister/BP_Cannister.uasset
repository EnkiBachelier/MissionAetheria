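; BP_Cannister is a canister actor that visually shows a replicated fill level.
; BeginPlay creates dynamic material instances for the static mesh's materials.
; OnRep_FillAmount calls ChangeFillAmount when the value changes, which loops past the first material and starts a timeline to drive the FillAmount scalar parameter.
; The timeline updates LastFillAmount as it lerps toward the target, then snaps to the exact value on finish.
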(event Custom|ChangeFillAmount
  (for (_array_element _array_index) (Variables|Default|GetMaterialInsideCan)
    (if (> _array_index 0)
      (bind _alpha (Timeline|Timeline PlayFromStart)
        (:Update
          (Rendering|Material|SetScalarParameterValue _array_element "FillAmount" (Math|Float|Lerp (Variables|Default|GetLastFillAmount) (Variables|Default|GetFillAmount) _alpha) :!class /Script/Engine.MaterialInstanceDynamic)
          (Variables|Default|SetLastFillAmount (Math|Float|Lerp (Variables|Default|GetLastFillAmount) (Variables|Default|GetFillAmount) _alpha)))
        (:Finished
          (Rendering|Material|SetScalarParameterValue _array_element "FillAmount" (Variables|Default|GetFillAmount) :!class /Script/Engine.MaterialInstanceDynamic)
          (Variables|Default|SetLastFillAmount (Variables|Default|GetFillAmount)))))))

(event EventBeginPlay
  (bind _staticmesh (Variables|Default|GetStaticMesh))
  (for (_array_element _array_index) (Rendering|Material|GetMaterials _staticmesh)
    (bind _returnvalue (Rendering|Material|CreateDynamicMaterialInstance _staticmesh _array_index _array_element "None" :!class /Script/Engine.PrimitiveComponent))
    (Utilities|Array|SetArrayElem (Variables|Default|GetMaterialInsideCan) _array_index _returnvalue true)))

(fn ConstructionScript)

(fn OnRepFillAmount
  (if (!= (Variables|Default|GetFillAmount) (Variables|Default|GetLastFillAmount))
    (CallFunction|ChangeFillAmount)))