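; Wwise music manager that plays menu, stage choice and battle music from a single event driven by music and combat state switches.
; PlayMusic restarts the event on a state change or when nothing is playing, inserting transition states between normal and losing combat music.
; The OnEndMusic callback replays looping states, resolves transitions to their target, and asks the cached GS_BaseStage to re-evaluate battle music after intro or normal segments.
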(event Custom|OnEndMusic
  (params (CallbackType :type EAkCallbackType%20Enum :default "EndOfEvent") (CallbackInfo :type Ak%20Callback%20Info%20Object%20Reference))
  (Variables|Default|SetisPlayingMusic false)
  (switch Utilities|FlowControl|Switch|SwitchonEnum_MusicState (Variables|Default|GetCurrent%20Music%20State)
    (:NewEnumerator0
      (CallFunction|PlayMusic (Variables|Default|GetCurrent%20Music%20State) "NewEnumerator4" false :!label _label))
    (:NewEnumerator1
      (goto _label))
    (:NewEnumerator2
      (switch Utilities|FlowControl|Switch|SwitchonBattleState (Variables|Default|GetCurrent%20Battle%20State)
        (:NewEnumerator2
          (CallFunction|PlayMusic "NewEnumerator2" (Variables|Default|GetCurrent%20Battle%20State) false :!label _label_2))
        (:NewEnumerator3
          (goto _label_2))
        (:NewEnumerator4
          (bind _asgs_base_stage (Utilities|GetGameStateBaseStage :!label _label_3)
            (:Valid
              (bind _output_get (Variables|Default|SetCurrent%20Battle%20State "NewEnumerator6"))
              (Default|BattleMusic _asgs_base_stage _output_get))
            (:NotValid
              (CallFunction|PlayMusic "NewEnumerator2" "NewEnumerator5" false))))
        (:NewEnumerator5
          (goto _label_3))
        (:NewEnumerator7
          (CallFunction|PlayMusic "NewEnumerator2" "NewEnumerator5" false))
        (:NewEnumerator8
          (CallFunction|PlayMusic "NewEnumerator2" "NewEnumerator2" false))))))

(event EventBeginPlay)

(event Collision|EventActorBeginOverlap
  (params (OtherActor :type Actor%20Object%20Reference)))

(event EventTick
  (params (DeltaSeconds :type Float%20%28single-precision%29)))

(fn ConstructionScript)

(fn PlayMusic
  (params (MusicState :type Enum_MusicState%20Enum :default "NewEnumerator0") (BattleState :type BattleState%20Enum :default "NewEnumerator0") (OverrideMusic :type Boolean))
  (if (and (Math|Boolean|ORBoolean (Utilities|Enum|NotEqual(Enum) MusicState (Variables|Default|GetCurrent%20Music%20State)) (Utilities|Enum|NotEqual(Enum) BattleState (Variables|Default|GetCurrent%20Battle%20State)) (not (Variables|Default|GetisPlayingMusic))) (Utilities|Enum|NotEqual(Enum) BattleState "NewEnumerator6"))
    (Class|AkGameObject|Stop (Variables|Default|GetAk))
    (Variables|Default|SetCurrent%20Music%20State MusicState)
    (LocalVariables|SetMusicSwitch (Utilities|Select :Index (Variables|Default|GetCurrent%20Music%20State) :NewEnumerator0 "/Game/WwiseAudio/Switches/Default_Work_Unit/MusicState/MusicState-MENU.MusicState-MENU" :NewEnumerator1 "/Game/WwiseAudio/Switches/Default_Work_Unit/MusicState/MusicState-STAGE_CHOICE.MusicState-STAGE_CHOICE" :NewEnumerator2 "/Game/WwiseAudio/Switches/Default_Work_Unit/MusicState/MusicState-COMBAT.MusicState-COMBAT"))
    (Class|AkComponent|SetSwitch (Variables|Default|GetAk) (LocalVariables|GetMusicSwitch) "MusicState")
    (switch Utilities|FlowControl|Switch|SwitchonEnum_MusicState (Variables|Default|GetCurrent%20Music%20State)
      (:NewEnumerator0
        _)
      (:NewEnumerator1
        _)
      (:NewEnumerator2
        (LocalVariables|SetBattleStateWanted BattleState)
        ;[1 1 1] SetNormalToLoosing
        (if (and (or (Utilities|Enum|Equal(Enum) (Variables|Default|GetCurrent%20Battle%20State) "NewEnumerator5") (Utilities|Enum|Equal(Enum) (Variables|Default|GetCurrent%20Battle%20State) "NewEnumerator6")) (Utilities|Enum|Equal(Enum) BattleState "NewEnumerator2"))
          (Variables|Default|SetCurrent%20Battle%20State "NewEnumerator8")
          (else
            ;[1 1 1] SetLoosingToNormal
            (if (and (Utilities|Enum|Equal(Enum) (Variables|Default|GetCurrent%20Battle%20State) "NewEnumerator2") (Utilities|Enum|Equal(Enum) BattleState "NewEnumerator5"))
              (Variables|Default|SetCurrent%20Battle%20State "NewEnumerator7")
              (else
                (Variables|Default|SetCurrent%20Battle%20State (LocalVariables|GetBattleStateWanted))))))
        (bind _output_get (LocalVariables|SetBattleSwitch (Utilities|Select :Index (Variables|Default|GetCurrent%20Battle%20State) :NewEnumerator0 "/Game/WwiseAudio/Switches/Default_Work_Unit/CombatState/CombatState-WON.CombatState-WON" :NewEnumerator1 "/Game/WwiseAudio/Switches/Default_Work_Unit/CombatState/CombatState-LOST.CombatState-LOST" :NewEnumerator2 "/Game/WwiseAudio/Switches/Default_Work_Unit/CombatState/CombatState-LOSING.CombatState-LOSING" :NewEnumerator3 "/Game/WwiseAudio/Switches/Default_Work_Unit/CombatState/CombatState-WINNING.CombatState-WINNING" :NewEnumerator4 "/Game/WwiseAudio/Switches/Default_Work_Unit/CombatState/CombatState-INTRO.CombatState-INTRO" :NewEnumerator5 "/Game/WwiseAudio/Switches/Default_Work_Unit/CombatState/CombatState-NORMAL.CombatState-NORMAL" :NewEnumerator7 "/Game/WwiseAudio/Switches/Default_Work_Unit/CombatState/CombatState-LOSING_TO_NORMAL.CombatState-LOSING_TO_NORMAL" :NewEnumerator8 "/Game/WwiseAudio/Switches/Default_Work_Unit/CombatState/CombatState-NORMAL_TO_LOSING.CombatState-NORMAL_TO_LOSING" :NewEnumerator6 0)))
        (Class|AkComponent|SetSwitch (Variables|Default|GetAk) _output_get "CombatState")))
    (Class|AkGameObject|PostAkEvent (Variables|Default|GetAk) "/Game/WwiseAudio/Events/Default_Work_Unit/Music.Music" 4 (EventDispatchers|CreateEvent :!event Custom|OnEndMusic))
    (Variables|Default|SetisPlayingMusic true)))