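; Base robot enemy AI for range, melee and drone types, reading health and attack damage from a data table.
; It takes player damage and timer-driven fire and burn ticks, while RepNotify material parameters drive hit flashes and a dissolve.
; Attack fires a randomly offset line-traced Niagara laser at the blackboard target, damaging players unless shielded.
; On death it broadcasts the kill and is deactivated rather than destroyed, with SetInUse toggling collision, visibility and brain logic.
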(event Custom|SetDissolveState
  (bind _materialrobot (CallFunction|GetMaterialRobot))
  (bind _lastdissolvestate (Variables|Default|GetLastDissolveState))
  ;[1 1 1] Set Dissolve State
  (bind _dissolveeffect (Timeline|DissolveTimeline PlayFromStart)
    (:Update
      (for (_array_element _array_index) _materialrobot
        (if (and (Utilities|IsValid _array_element) (Utilities|Array|IsValidIndex _lastdissolvestate _array_index))
          (Rendering|Material|SetScalarParameterValue _array_element "DissolveAmount" (Math|Float|Lerp (Utilities|Array|Get(acopy) _lastdissolvestate _array_index) (Variables|Default|GetDissolveState) _dissolveeffect) :!class /Script/Engine.MaterialInstanceDynamic))))
    (:Finished
      (for (_array_element_2 _array_index_2) _materialrobot
        (if (and (Utilities|IsValid _array_element_2) (Utilities|Array|IsValidIndex (Variables|Default|GetLastDissolveState) _array_index_2))
          (Rendering|Material|SetScalarParameterValue _array_element_2 "DissolveAmount" (Variables|Default|GetDissolveState) :!class /Script/Engine.MaterialInstanceDynamic)
          (Utilities|Array|SetArrayElem (Variables|Default|GetLastDissolveState) _array_index_2 (Variables|Default|GetDissolveState)))))))

(event Custom|InFireTick
  ;[1 1 1] Burn system
  (if (Variables|Burn|GetIsInFire)
    (Game|Damage|ApplyDamage self (Variables|Burn|GetFireDamage) 0 0 "/Script/Engine.DamageType")
    (else
      (Utilities|Time|ClearandInvalidateTimerbyHandle (Variables|Burn|GetTimerInFireHandle))
      (Variables|Burn|SetBurnTicksAmount 4)
      (bind _returnvalue (Utilities|Time|SetTimerbyEvent (delegate Custom|BurnTick) (Variables|Burn|GetBurnTicksDelay) true))
      (Variables|Burn|SetTimerBurningHandle _returnvalue))))

(event Custom|Server_Attack
  (params (IndexAnimAttack :type Integer))
  (CallFunction|Attack IndexAnimAttack))

(event Custom|BurnTick
  ;[1 1 1] Burn system
  (if (<= (Variables|Burn|GetBurnTicksAmount) 0)
    (Utilities|Time|ClearandInvalidateTimerbyHandle (Variables|Burn|GetTimerBurningHandle))
    (else
      (Variables|Burn|SetBurnTicksAmount (- (Variables|Burn|GetBurnTicksAmount) 1))
      (Game|Damage|ApplyDamage self (Variables|Burn|GetBurnDamage) 0 0 "/Script/Engine.DamageType"))))

(event EventDealDamage
  (params (damagesToDeal :type Float%20%28double-precision%29) (Actor%20Type :type Enum_ActorType%20Enum :default "NewEnumerator0") (DamageCauser :type Actor%20Object%20Reference))
  ;[1 1 1] Deal Damage to self
  (if (Variables|Default|GetIsEnabled)
    (switch Utilities|FlowControl|Switch|SwitchonEnum_ActorType Actor%20Type
      (:NewEnumerator0
        (Game|Damage|ApplyDamage self damagesToDeal 0 DamageCauser "/Script/Engine.DamageType"))
      (:NewEnumerator1
        (Development|PrintString "A friend of yours bip bouped you. That's not cool, you should remind him that you are together in this war (Even if in the end it doesn't even matter)")))))

(event Game|Damage|EventAnyDamage
  (params (Damage :type Float%20%28single-precision%29) (DamageType :type Damage%20Type%20Object%20Reference) (InstigatedBy :type Controller%20Object%20Reference) (DamageCauser :type Actor%20Object%20Reference))
  ;[1 1 1] Health update
  (if (not (Variables|Default|GetIsDead))
    (bind _output_get (Variables|Default|SetCurrentHealth (- (Variables|Default|GetCurrentHealth) Damage)))
    (Variables|Default|SetCurrentEmmisiveColor (Variables|Default|GetColorValue))
    (Utilities|FlowControl|Sequence
      (:then_0
        (Default|CallOnAIHIt)
        (Utilities|FlowControl|Delay 0.2)
        (Variables|Default|SetCurrentEmmisiveColor (Variables|Default|GetDefaultColorValue)))
      (:then_1
        (if (<= _output_get 0.0)
          (Variables|Default|SetIsDead true)
          (Variables|/Script/Engine.CharacterMovementComponent|SetMaxWalkSpeed (Variables|Character|GetCharacterMovement) 0.0)
          (Variables|Default|SetDissolveState 0.7)
          (CallFunction|OnKilled)
          (Variables|Default|SetdeathLocation (Transformation|GetActorLocation self))
          (Utilities|FlowControl|Delay 2.0)
          (CallFunction|SetinUse false)
          (bind _asbp_base_playable_character (Utilities|Casting|CastToBP_BasePlayableCharacter DamageCauser)
            (:then
              _)
            (:CastFailed
              _))
          (Default|CallOnAIKilled self _asbp_base_playable_character (Variables|Default|GetdeathLocation)))))))

(event EventBurn
  (params (AttackerType :type Enum_ActorType%20Enum :default "NewEnumerator0") (IsInFire :type Boolean))
  ;[1 1 1] Burn system
  (switch Utilities|FlowControl|Switch|SwitchonEnum_ActorType AttackerType
    (:NewEnumerator0
      (Variables|Burn|SetIsInFire IsInFire)
      (if (not (Utilities|Time|IsTimerActivebyHandle (Variables|Burn|GetTimerInFireHandle)))
        (bind _returnvalue (Utilities|Time|SetTimerbyEvent (delegate Custom|InFireTick) (Variables|Burn|GetFireTicksDelay) true))
        (Variables|Burn|SetTimerInFireHandle _returnvalue)
        (Class|AkGameplayStatics|PostEvent "/Game/WwiseAudio/Events/Default_Work_Unit/SFX_Robots/LittleRobot/Play_little_robot_in_fire.Play_little_robot_in_fire" self)))))

(event EventBeginPlay
  ;[1 1 1] BeginPlay
  (Variables|Default|SetCurrentEmmisiveColor (Variables|Default|GetDefaultColorValue))
  (CallFunction|SetDissolveColor)
  (for _array_element (CallFunction|GetMaterialRobot)
    (Utilities|Array|AddUnique (Variables|Default|GetLastDissolveState) 0.0)))

(event EventSetinUse
  (params (InUse :type Boolean))
  (bind _aicontroller (CallFunction|GetAIContoller))
  (bind _braincomponent (Variables|/Script/AIModule.AIController|GetBrainComponent _aicontroller))
  ;[1 1 1] Set In Use
  (bind _output_get (Variables|Default|SetIsEnabled InUse))
  (Collision|SetActorEnableCollision _output_get)
  (Rendering|SetActorHiddenInGame (not _output_get))
  (if InUse
    (Variables|Default|SetDissolveState -0.4)
    (Variables|Default|SetIsDead false)
    (Class|BrainComponent|RestartLogic _braincomponent)
    (else
      (Transformation|SetActorLocation "-1000.000000,-1000.000000,-1000.000000" false false) ; Hotfix to avoid a frame where the collision is still active when a client kills an AI
      (AI|Logic|StopLogic _braincomponent "AI Deactivated"))))

(event EventEndPlay
  (params (EndPlayReason :type EEndPlayReason%20Enum :default "Destroyed"))
  ;[0.04167 0.04167 0.04167] EndPlay
  (EventDispatchers|UnbindallEventsfromOnAIKilled))

(fn ConstructionScript
  (bind _returnvalue (Utilities|GetDataTableRow "/Game/MissionAetheria/Datatables/DataTable_AI.DataTable_AI" (Utilities|Select :Index (Variables|Default|GetTypeAI) :NewEnumerator0 "Range" :NewEnumerator1 "Melee" :NewEnumerator2 "Drone"))
    (:then
      (bind _output_get (Variables|Default|SetData _returnvalue))
      (Variables|Default|SetCurrentHealth (.maxhealth _output_get)))
    (:RowNotFound
      (Development|PrintString "Data Table Row not found in BP_AI (Construction Script)"))))

(fn UpdateWalkSpeed
  (params (New%20Walk%20Speed :type Float%20%28double-precision%29))
  (Variables|/Script/Engine.CharacterMovementComponent|SetMaxWalkSpeed (Variables|Character|GetCharacterMovement) New%20Walk%20Speed))

(fn OnRepCurrentEmmisiveColor
  (for _array_element (CallFunction|GetMaterialRobot)
    (Utilities|IsValid _array_element
      (:Is%20Valid
        (Rendering|Material|SetScalarParameterValue _array_element "EmissiveColor" (Variables|Default|GetCurrentEmmisiveColor) :!class /Script/Engine.MaterialInstanceDynamic))
      (:Is%20Not%20Valid
        (Development|PrintString "MATERIAL ROBOT NOT VALID (rep_currentEmissive)")))))

(fn OnRepDissolveState
  (for _array_element (Variables|Default|GetLastDissolveState)
    (if (!= (Variables|Default|GetDissolveState) _array_element)
      (CallFunction|SetDissolveState))))

(fn SetDissolveColor
  (for _array_element (CallFunction|GetMaterialRobot)
    (Rendering|Material|SetVectorParameterValue _array_element "DissolveColor" (Variables|Default|GetDissolveColor) :!class /Script/Engine.MaterialInstanceDynamic)))

(fn GetMaterialRobot
  (bind _mesh (Variables|Character|GetMesh))
  (bind _materialrobot (Variables|Default|GetMaterialRobot))
  (if (Utilities|Array|IsEmpty (Variables|Default|GetMaterialRobot))
    (for (_array_element _array_index) (Rendering|Material|GetMaterials _mesh)
      (bind _returnvalue (Rendering|Material|CreateDynamicMaterialInstance _mesh _array_index _array_element "None" :!class /Script/Engine.PrimitiveComponent))
      (Utilities|Array|AddUnique _materialrobot _returnvalue)
      (Utilities|Array|Add (Variables|Default|GetLastDissolveState) 0.0)))
  (return _materialrobot))

(fn Attack
  (params (IndexAnimAttack :type Integer))
  (bind _asactor (Utilities|Casting|CastToActor (AI|Components|Blackboard|GetValueasObject (Variables|/Script/AIModule.AIController|GetBlackboard (CallFunction|GetAIContoller)) (Variables|Default|GetTargetLocationName))))
  (bind _output_get (Variables|Default|SetTargetLocation (+ (Transformation|GetActorLocation _asactor) (Math|Vector|MakeVector (Math|Random|RandomFloatinRange (Variables|Default|GetMin) (Variables|Default|GetMax)) (Math|Random|RandomFloatinRange (Variables|Default|GetMin) (Variables|Default|GetMax)) (Math|Random|RandomFloatinRange (Variables|Default|GetMin) (Variables|Default|GetMax))))))
  (CallFunction|UpdateSpineRotation)
  (bind (_outhit _returnvalue) (Collision|LineTraceByChannel (Transformation|GetSocketLocation (Variables|Character|GetMesh) (Variables|Default|GetIn%20Socket%20Name)) _output_get "TraceTypeQuery2" true 0 "None" true "(R=1.000000,G=0.000000,B=0.000000,A=1.000000)" "(R=0.000000,G=1.000000,B=0.000000,A=1.000000)" 2.0))
  (bind _returnvalue_2 (Niagara|SpawnSystematLocation "/Game/MissionAetheria/VFX/Niagara/NS_LaserShoot.NS_LaserShoot" (.TraceStart (Collision|BreakHitResult _outhit)) (.rotation (Transformation|GetSocketTransform (Variables|Character|GetMesh) (Variables|Default|GetIn%20Socket%20Name) "RTS_World")) "1.000000,1.000000,1.000000" true true "AutoRelease"))
  (Niagara|SetNiagaraVariable(Vector3) _returnvalue_2 "StartLocation" (.TraceStart (Collision|BreakHitResult _outhit)))
  (if _returnvalue
    (Niagara|SetNiagaraVariable(Vector3) _returnvalue_2 "Target" (.Location (Collision|BreakHitResult _outhit)))
    (else
      (Niagara|SetNiagaraVariable(Vector3) _returnvalue_2 "Target" (.TraceEnd (Collision|BreakHitResult _outhit)))))
  (if (== (.HitActor (Collision|BreakHitResult _outhit)) "/Game/MissionAetheria/Blueprints/Abilities/Active/BP_Shield.BP_Shield")
    (Development|PrintString "Shield")
    (elif (and _returnvalue (Utilities|ClassIsChildOf (Utilities|GetClass (.HitActor (Collision|BreakHitResult _outhit))) "/Game/MissionAetheria/Blueprints/Player/BP_BasePlayableCharacter.BP_BasePlayableCharacter_C"))
      (Class|IDamageable|DealDamage(Message) (.HitActor (Collision|BreakHitResult _outhit)) (CallFunction|GetDamageAmount) "NewEnumerator1"))))

(fn GetDamageAmount
  (if (!= (Variables|Default|GetOut%20Row%20Damage%20Amount) -1.0)
    (return (Variables|Default|GetOut%20Row%20Damage%20Amount))
    (else
      (bind _returnvalue (Utilities|GetDataTableRow "/Game/MissionAetheria/Datatables/DataTable_AI.DataTable_AI" (Utilities|String|StringToName (Utilities|String|EnumtoString (Variables|Default|GetTypeAi))))
        (:then
          (bind _output_get (Variables|Default|SetOut%20Row%20Damage%20Amount (.damageamount _returnvalue)))
          (return (Variables|Default|GetOut%20Row%20Damage%20Amount)))
        (:RowNotFound
          (Development|PrintString "Hello"))))))

(fn UpdateSpineRotation
  (bind _returnvalue (Transformation|GetActorForwardVector))
  (bind _returnvalue_2 (Transformation|GetActorLocation))
  (bind _mesh (Variables|Character|GetMesh))
  (bind _targetlocation (Variables|Default|GetTargetlocation))
  (bind _returnvalue_3 (Math|Vector|Normalize (Math|Vector|MakeVector (.x _returnvalue) (.y _returnvalue) 0.0)))
  (bind _returnvalue_4 (Transformation|GetBoneTransform _mesh "Spine03" "RTS_ParentBoneSpace"))
  (bind _returnvalue_5 (- _targetlocation _returnvalue_2))
  (bind _returnvalue_6 (Math|Vector|Normalize (Math|Vector|MakeVector (.x _returnvalue_5) (.y _returnvalue_5) 0.0)))
  (bind _returnvalue_7 (Math|Vector|DotProduct _returnvalue_3 _returnvalue_6))
  (bind _returnvalue_8 (Class|KismetMathLibrary|DegAcos _returnvalue_7))
  (bind _returnvalue_9 (* _returnvalue_8 -1.0))
  (if (< (.z (Math|Vector|CrossProduct _returnvalue_3 _returnvalue_6)) 0.0)
    (bind _output_get (LocalVariables|SetAngle _returnvalue_9))
    (Variables|Default|SetRotateSpine (Math|Rotator|MakeRotator (.roll (.rotation _returnvalue_4)) (.pitch (.rotation _returnvalue_4)) (+ _returnvalue_9 _output_get -15.0)))
    (else
      (LocalVariables|SetAngle _returnvalue_8))))

(fn GetAIContoller
  (bind _returnvalue (Pawn|GetController))
  (Variables|Default|GetAIController
    (:then
      (return (Variables|Default|GetAIController)))
    (:else
      (bind _asaicontroller (Utilities|Casting|CastToAIController _returnvalue)
        (:then
          (Variables|Default|SetAIController _asaicontroller)
          (return (Variables|Default|GetAIController)))
        (:CastFailed
          (Development|PrintString (Utilities|GetDisplayName _returnvalue)))))))

(fn GetAttackRange
  (params (Player :type BP%20Base%20Playable%20Character%20Object%20Reference))
  (return (Variables|Default|GetAttackRange)))

(fn OnKilled
  (AI|Logic|StopLogic (Variables|/Script/AIModule.AIController|GetBrainComponent (CallFunction|GetAIContoller)) "AI Deactivated"))