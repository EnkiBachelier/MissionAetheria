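; BP_Player_Lobby is the lobby player class that puts the WBP_Lobby screen in front of the local player.
; On BeginPlay it creates the widget once if locally controlled, caches it, adds it to the player screen and focuses it.
; A getter lazily casts and caches the PC_Lobby controller.
; After unpausing, it restores UI-only input focused on the lobby widget.
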(event EventBeginPlay
  (|CallParentFunction)
  (CallFunction|ShowLobbyScreen))

(fn ConstructionScript)

(fn ShowLobbyScreen
  (bind _outplayercontroller (CallFunction|GetPlayerController))
  (Variables|Default|GetWBP_Lobby
    (:then
      (UserInterface|Viewport|AddtoPlayerScreen (Variables|Default|GetWBP_Lobby) :!label _label)
      (Widget|SetFocus (Variables|Default|GetWBP_Lobby)))
    (:else
      (Utilities|IsValid _outplayercontroller
        (:Is%20Valid
          (if (Pawn|IsLocallyControlled)
            (bind _returnvalue (UserInterface|CreateWidget "/Game/MissionAetheria/UI/Lobby/WBP_Lobby.WBP_Lobby_C" _outplayercontroller))
            (Variables|Default|SetWBP_Lobby _returnvalue)
            (goto _label)))))))

(fn GetPlayerController
  (Utilities|IsValid (Variables|Default|GetPlayerController)
    (:Is%20Valid
      _)
    (:Is%20Not%20Valid
      (bind _aspc_lobby (Utilities|Casting|CastToPC_Lobby (Game|GetPlayerController 0)))
      (Variables|Default|SetPlayerController _aspc_lobby)))
  (return (Variables|Default|GetPlayerController)))

(fn AfterSetPause
  (params (IsPaused :type Boolean))
  (bind _outplayercontroller (CallFunction|GetPlayerController))
  (|CallParentFunction IsPaused)
  (if (not IsPaused)
    (Utilities|IsValid _outplayercontroller
      (:Is%20Valid
        (Input|SetInputModeUIOnly _outplayercontroller (Variables|Default|GetWBP_Lobby) "DoNotLock" false)))))