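; Base player controller for Mission Aetheria stages, acting as the network hub between local players and server game logic.
; On BeginPlay, the local controller requests its pawn spawn, creates the role-based stage HUD and registers input mapping contexts.
; Server events apply damage, resurrection and missile hits, or relay effects through GameState and boosts, end screens and outcomes through client events.
; Completed levels are copied from the server's GameInstance to clients, since it is not replicated.
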(event Custom|Server_AttachToPilot
  (params (isAttached :type Boolean))
  ;[0.03646 0.03646 0.03646] AttachToPilot
  (Default|ClientAttachtoPilot (CallFunction|GetGameState) isAttached))

(event Custom|Server_SwitchLevel
  (params (newLevelName :type String))
  ;[0.03646 0.03646 0.03646] SwitchLevel
  (Development|PrintString "player controller switch level")
  (Default|ClientonSwitchLevel (CallFunction|GetGameState) newLevelName))

(event Custom|Server_ShowEndScreen
  (params (hasWon :type Boolean) (IsEndless :type Boolean) (NumberWavesSurvived :type Integer))
  ;[0.05208 0.05208 0.05208] EndScreen
  (CallFunction|ClientShowEndScreen hasWon IsEndless NumberWavesSurvived))

(event Custom|Client_BoostCharacterData
  (params (boostType :type Enum_CharacterBoostType%20Enum :default "NewEnumerator0") (multiplier :type Float%20%28double-precision%29) (duration :type Float%20%28double-precision%29) (shouldDivide :type Boolean))
  ;[0.05208 0.05208 0.05208] BoostCharacterData
  (Default|BoostCharacterData (CallFunction|GetPlayerPawn) boostType multiplier duration shouldDivide false))

(event Custom|Client_ShowEndScreen
  (params (hasWon :type Boolean) (IsEndless :type Boolean) (NumberWavesSurvived :type Integer))
  ;[0.05208 0.05208 0.05208] EndScreen
  (bind _returnvalue (UserInterface|CreateWidget "/Game/MissionAetheria/UI/Stages/WBP_EndStageScreen.WBP_EndStageScreen_C"))
  (UserInterface|Viewport|AddtoPlayerScreen _returnvalue)
  (Default|SetState _returnvalue hasWon IsEndless)
  (if IsEndless
    (Default|SetNumberWavesSurvived _returnvalue NumberWavesSurvived)))

(event Custom|Server_OnMissileHit
  (params (missile :type BP%20Missile%20Object%20Reference) (radius :type Float%20%28double-precision%29))
  (bind _returnvalue (Transformation|GetActorLocation missile))
  ;[0.08333 0.08333 0.08333] OnMissileHit
  (Game|Damage|ApplyRadialDamage 5.0 _returnvalue radius "/Game/MissionAetheria/Blueprints/Damages/BP_Damage_Pilot_Missile.BP_Damage_Pilot_Missile_C" 0 missile 0 false "ECC_Visibility")
  (Default|ClientonMissileHit (CallFunction|GetGameState) _returnvalue)
  (Default|OnMissileHit missile))

(event Custom|Server_ShowMuzzleShotVFX
  (params (Sender :type Enum_CharacterRoles%20Enum :default "NewEnumerator5") (IsActive :type Boolean))
  ;[0.05208 0.05208 0.05208] MuzzleShotVisibility
  (Default|ClientShowMuzzleShotVFX (CallFunction|GetGameState) Sender IsActive))

(event Custom|Server_SavePlayedLevelOutcome
  (params (hasWon :type Boolean))
  (bind _gameinstance (CallFunction|GetGameInstance))
  ;[0.05208 0.05208 0.05208] EndScreen
  (Default|SavePlayedLevelOutcome _gameinstance hasWon) ; GI is not replicated so we change the value on the server & copy the whole thing to the \nclients (we can't tell all the clients to save the value)
  (CallFunction|ClientSavePlayedLevelOutcome (Variables|/Game/MissionAetheria/Blueprints/GameInstance/GI_MissionAetheria.GI_MissionAetheria_C|GetCompletedLevelsRowName _gameinstance)))

(event Custom|Client_SavePlayedLevelOutcome
  (params (completedLevelNames :type Array%20of%20Names))
  ;[0.05208 0.05208 0.05208] EndScreen
  (Variables|/Game/MissionAetheria/Blueprints/GameInstance/GI_MissionAetheria.GI_MissionAetheria_C|SetCompletedLevelsRowName (CallFunction|GetGameInstance) completedLevelNames))

(event Custom|Server_SpawnPlayer
  (params (Player :type Struct%20Player%20Structure))
  ;[0.03125 0.03125 0.03125] SpawnPlayer
  (Default|SpawnPlayer (CallFunction|GetGameMode) self Player))

(event Custom|Server_DealDamage
  (params (Damage :type Float%20%28double-precision%29) (Target :type I%20Damageable%20Interface) (IsBurnDamage :type Boolean) (IsOverlap :type Boolean) (DamageCauser :type Actor%20Object%20Reference))
  (bind _returnvalue (Utilities|ToObject(Interface) Target))
  ;[0.03125 0.03125 0.03125] DealDamage
  (if IsBurnDamage
    (Class|IDamageable|Burn(Message) _returnvalue "NewEnumerator0" IsOverlap)
    (else
      (Class|IDamageable|DealDamage(Message) _returnvalue Damage "NewEnumerator0" DamageCauser))))

(event Custom|Server_BoostCharacterData
  (params (boostType :type Enum_CharacterBoostType%20Enum :default "NewEnumerator0") (multiplier :type Float%20%28double-precision%29) (duration :type Float%20%28double-precision%29) (shouldDivide :type Boolean) (Target :type Actor%20Object%20Reference))
  ;[0.05208 0.05208 0.05208] BoostCharacterData
  (CallFunction|ClientBoostCharacterData boostType multiplier duration shouldDivide)
  (Actor|DestroyActor Target))

(event Custom|Server_OnPlayerDamaged
  (params (player :type BP%20Base%20Playable%20Character%20Object%20Reference) (damageAmount :type Float%20%28double-precision%29))
  ;[0.05208 0.05208 0.05208] EndScreen
  (Default|ClientonPlayerDamaged (CallFunction|GetGameState) player)
  (Game|Damage|ApplyDamage player damageAmount 0 0 "/Script/Engine.DamageType"))

(event Custom|Server_Resurrect
  (params (Target :type Actor%20Object%20Reference) (PlayerHelper :type BP%20Base%20Playable%20Character%20Object%20Reference))
  ;[0.03125 0.03125 0.03125] Resurrect
  (Class|IHealable|Resurrect(Message) Target PlayerHelper))

(event EventBeginPlay
  (bind _gameinstance (CallFunction|GetGameInstance))
  (bind _returnvalue (CallFunction|GetUserSettings))
  (bind _currentplayer (Variables|/Game/MissionAetheria/Blueprints/GameInstance/GI_MissionAetheria.GI_MissionAetheria_C|GetCurrentPlayer _gameinstance))
  ;[0.06771 0.06771 0.06771] BeginPlay
  (if (Pawn|IsLocalPlayerController)
    (CallFunction|ServerSpawnPlayer _currentplayer)
    (bind _returnvalue_2 (UserInterface|CreateWidget "/Game/MissionAetheria/UI/Stages/WBP_Stage_General.WBP_Stage_General_C" 0 (.Role (Utilities|Struct|BreakStruct_Player _currentplayer)) (Variables|/Game/MissionAetheria/Blueprints/GameStates/GS_BaseStage.GS_BaseStage_C|GetTypeStage (CallFunction|GetGameState))))
    (bind _output_get (Variables|Default|SetWBPStageGeneral _returnvalue_2))
    (UserInterface|Viewport|AddtoPlayerScreen _output_get)
    (Input|SetInputModeGameOnly self false)
    (for _array_element (CallFunction|GetAllIMC)
      (if (not (Class|EnhancedInputUserSettings|IsMappingContextRegistered _returnvalue _array_element))
        (Class|EnhancedInputUserSettings|RegisterInputMappingContext _returnvalue _array_element)))))

(fn ConstructionScript)

(fn GetGameMode
  (Variables|Default|GetGameMode
    (:then
      _)
    (:else
      (bind _asgm_base_stage (Utilities|Casting|CastToGM_BaseStage (Game|GetGameMode)))
      (Variables|Default|SetGameMode _asgm_base_stage)))
  (return (Variables|Default|GetGameMode)))

(fn GetGameInstance
  (Variables|Default|GetGameInstance
    (:then
      _)
    (:else
      (bind _asgi_mission_aetheria (Utilities|Casting|CastToGI_MissionAetheria (Game|GetGameInstance)))
      (Variables|Default|SetGameInstance _asgi_mission_aetheria)))
  (return (Variables|Default|GetGameInstance)))

(fn GetPlayerPawn
  (Variables|Default|GetPlayableCharacter
    (:then
      _)
    (:else
      (bind _asbp_base_playable_character (Utilities|Casting|CastToBP_BasePlayableCharacter (Game|Player|GetPlayerPawn 0)))
      (Variables|Default|SetPlayableCharacter _asbp_base_playable_character)))
  (return (Variables|Default|GetPlayableCharacter)))

(fn GetGameState
  (Utilities|IsValid (Variables|Default|GetgameState)
    (:Is%20Valid
      _)
    (:Is%20Not%20Valid
      (bind _asgs_base_stage (Utilities|Casting|CastToGS_BaseStage (Game|GetGameState)))
      (Variables|Default|SetgameState _asgs_base_stage)))
  (return (Variables|Default|GetgameState)))

(fn UpdateCannister
  (params (CurrentHp :type Float%20%28double-precision%29) (Role :type Enum_CharacterRoles%20Enum :default "NewEnumerator5"))
  (Default|UpdateCannister (Variables|Default|GetWBPStageGeneral) CurrentHp Role))

(fn EnableAbility
  (params (IsEnable :type Boolean))
  (Default|EnableAbility (Variables|Default|GetWBPStageGeneral) IsEnable))