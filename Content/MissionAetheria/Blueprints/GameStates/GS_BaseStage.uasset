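; Base GameState for stages, holding player count, stage type, characters in game and living players, copied from the GameInstance through Server events.
; Client events handle level switching, pilot attraction, hit screens, muzzle flashes and missile explosions.
; BattleMusic picks the music state from battle outcome, living-player count and wave progress.
; Helpers return random players or find characters by role, with the Pilot reference cached after lookup.
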(event Custom|Client_AttachToPilot
  (params (isAttached :type Boolean))
  (bind _pilot (Utilities|GetPilotCharacter)
    (:Valid
      (Variables|/Game/MissionAetheria/Blueprints/Player/PlayableCharacters/BP_PlayableCharacter_Pilot.BP_PlayableCharacter_Pilot_C|SetCanAttractCharacter _pilot isAttached)
      (Default|UpdatePilotCollisionSize _pilot))))

(event Custom|Player%20List%20Add
  (params (Player :type Character%20Object%20Reference%20%28by%20ref%29))
  (Utilities|Array|Add (Variables|Default|GetPlayerList) Player))

(event Custom|Server_SetTypeStage
  (params (TypeStage :type Enum_StagesType%20Enum :default "NewEnumerator0"))
  (Variables|Default|SetTypeStage TypeStage))

(event Custom|Client_OnPlayerDamaged
  (params (playerDamaged :type BP%20Base%20Playable%20Character%20Object%20Reference))
  (bind _asbp_base_playable_character (Utilities|Casting|CastToBP_BasePlayableCharacter (Game|Player|GetPlayerPawn 0)))
  (if (== _asbp_base_playable_character playerDamaged)
    (bind _returnvalue (UserInterface|CreateWidget "/Game/MissionAetheria/UI/Combat/WBP_HitScreen.WBP_HitScreen_C"))
    (UserInterface|Viewport|AddtoPlayerScreen _returnvalue -20)))

(event Custom|Client_OnSwitchLevel
  (params (newLevelName :type String))
  (Default|SwitchLevel (CallFunction|GetGameInstance) newLevelName))

(event Custom|Server_SetCurrentNumberOfPlayer
  (params (CurrentNumberOfPlayer :type Integer))
  (Variables|Default|SetCurrentNumberOfPlayers CurrentNumberOfPlayer))

(event Custom|Server_SetCharacterInGame
  (params (Players :type Array%20of%20BP%20Base%20Playable%20Character%20Object%20References))
  (Variables|Default|SetCharacterInGame Players))

(event Custom|Server_SetPlayersAlive
  (params (PlayersAlive :type Array%20of%20BP%20Base%20Playable%20Character%20Object%20References))
  (Variables|Default|SetPlayersAlive PlayersAlive))

(event Custom|On%20Update%20Players%20Alives
  (params (PlayersAlivesArray :type Array%20of%20BP%20Base%20Playable%20Character%20Object%20References))
  (CallFunction|ServerSetPlayersAlive PlayersAlivesArray))

(event Custom|Client_ShowMuzzleShotVFX
  (params (Sender :type Enum_CharacterRoles%20Enum :default "NewEnumerator5") (IsActive :type Boolean))
  (for _array_element (Variables|Default|GetCharacterInGame)
    (Utilities|IsValid _array_element
      (:Is%20Valid
        (if (Utilities|Enum|Equal(Enum) Sender (Utilities|Struct|BreakStruct_CharacterData (Variables|/Game/MissionAetheria/Blueprints/Player/BP_BasePlayableCharacter.BP_BasePlayableCharacter_C|GetCharacterDatas _array_element)))
          (Default|ShowMuzzleShotVFX _array_element IsActive))))))

(event Custom|Client_OnMissileHit
  (params (location :type Vector))
  (Niagara|SpawnSystematLocation "/Game/MissionAetheria/VFX/Niagara/NS_MissileExplosion.NS_MissileExplosion" location "0, 0, 0" "1.000000,1.000000,1.000000" true true "AutoRelease"))

(event EventBeginPlay
  (bind _gameinstance (CallFunction|GetGameInstance))
  (|CallParentFunction)
  (CallFunction|ServerSetCurrentNumberOfPlayer (Variables|/Game/MissionAetheria/Blueprints/GameInstance/GI_MissionAetheria.GI_MissionAetheria_C|GetCurrentNumberOfPlayers _gameinstance))
  (CallFunction|ServerSetTypeStage (Utilities|Struct|BreakStruct_LevelData (Variables|/Game/MissionAetheria/Blueprints/GameInstance/GI_MissionAetheria.GI_MissionAetheria_C|GetLevelData _gameinstance)))
  (CallFunction|ServerSetCharacterinGame (Variables|/Game/MissionAetheria/Blueprints/GameInstance/GI_MissionAetheria.GI_MissionAetheria_C|GetCharactersInGame (CallFunction|GetGameInstance)))
  (EventDispatchers|BindEventtoUpdatePlayersAlive (CallFunction|GetGameInstance) (delegate Custom|On%20Update%20Players%20Alives)))

(fn ConstructionScript)

(fn FindPlayerinArraywithRole
  (params (Role :type Enum_CharacterRoles%20Enum :default "NewEnumerator5") (PlayerArray :type Array%20of%20BP%20Base%20Playable%20Character%20Object%20References))
  (bind _array_element (Utilities|Array|ForEachLoopwithBreak PlayerArray)
    (:LoopBody
      (if (Utilities|Enum|Equal(Enum) (.characterrole (Variables|/Game/MissionAetheria/Blueprints/Player/BP_BasePlayableCharacter.BP_BasePlayableCharacter_C|GetCharacterDatas _array_element)) Role)
        (LocalVariables|SetPlayerFoundInArray _array_element)))
    (:Completed
      (return (LocalVariables|GetPlayerFoundInArray)))))

(fn GetPiloteinGame
  (if (Variables|Default|GetGameHasPilot)
    (Variables|Default|GetPiloteInGame
      (:then
        _)
      (:else
        (bind _playerfound (CallFunction|FindPlayerinArraywithRole "NewEnumerator0" (Variables|Default|GetCharacterInGame)))
        (bind _asbp_playable_character_pilot (Utilities|Casting|CastToBP_PlayableCharacter_Pilot _playerfound))
        (Variables|Default|SetPiloteInGame _asbp_playable_character_pilot)))
    (return (Variables|Default|GetPiloteInGame))))

(fn BattleMusic
  (params (BattleState :type BattleState%20Enum :default "NewEnumerator0"))
  (bind _gameinstance (Variables|Default|GetGameInstance))
  (if (Utilities|Select :Index BattleState :NewEnumerator0 true :NewEnumerator1 true :NewEnumerator2 false :NewEnumerator3 false :NewEnumerator4 false :NewEnumerator5 false :NewEnumerator7 false :NewEnumerator8 false :NewEnumerator6 false)
    (CallFunction|HandleMusic "NewEnumerator2" "NewEnumerator0")
    (elif (Utilities|Select :Index (Variables|/Game/MissionAetheria/Blueprints/Sounds/BP_WwiseMusicManager.BP_WwiseMusicManager_C|GetCurrent%20Battle%20State (Variables|Default|GetMusicManagerRef)) :NewEnumerator0 false :NewEnumerator1 false :NewEnumerator2 true :NewEnumerator3 true :NewEnumerator4 false :NewEnumerator5 true :NewEnumerator7 true :NewEnumerator8 true :NewEnumerator6 true)
      (if (< (Utilities|Array|Length (Variables|Default|GetPlayersAlive)) 2)
        (CallFunction|HandleMusic "NewEnumerator2" "NewEnumerator2")
        (elif (<= (Variables|/Game/MissionAetheria/Blueprints/GameInstance/GI_MissionAetheria.GI_MissionAetheria_C|GetCurrentWaveIndex _gameinstance) (Math|Float|Floor (* (Math|Conversions|ToFloat(Integer) (Utilities|Array|Length (Utilities|Struct|BreakStruct_LevelData (Variables|/Game/MissionAetheria/Blueprints/GameInstance/GI_MissionAetheria.GI_MissionAetheria_C|GetLevelData _gameinstance)))) 0.75)))
          (CallFunction|HandleMusic "NewEnumerator2" "NewEnumerator3")
          (else
            (CallFunction|HandleMusic "NewEnumerator2" "NewEnumerator5")))))))

(fn GetRandomPlayersAlive
  (return (.OutItem (Utilities|Array|Random (Variables|Default|GetPlayersAlive)))))

(fn GetRandomCharacterinGame
  (return (.OutItem (Utilities|Array|Random (Variables|Default|GetCharacterInGame)))))