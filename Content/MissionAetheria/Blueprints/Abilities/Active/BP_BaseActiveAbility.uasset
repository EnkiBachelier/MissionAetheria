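; Base class for active player abilities, providing use gating, reload timing and empty hooks for VFX visibility and animation notifies.
; TryToUse clears the ready flag and calls the overridable Use, which flags the owner as using an ability through a server call.
; OnReload notifies the owner, clears that state and restores readiness after ReloadDuration.
; A RepNotify forwards VFX visibility to the owner's server call, and a getter lazily caches the first player controller.
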(event Custom|OnReload
  (CallFunction|PlayerReloadAbility)
  (Utilities|FlowControl|Delay (Variables|Default|GetReloadDuration))
  (Variables|Default|SetIsReadyToBeUsed true))

(fn ConstructionScript)

(fn TrytoUse
  (if (Variables|Default|GetIsReadyToBeUsed)
    (Variables|Default|SetIsReadyToBeUsed false)
    (CallFunction|Use)))

(fn Use
  (Default|ServerSetIsUsingAbility (Variables|Default|GetPlayerOwner) true))

(fn PlayerUseAbility
  (bind _playerowner (Variables|Default|GetPlayerOwner))
  (Utilities|IsValid _playerowner
    (:Is%20Valid
      (Default|UseAbility _playerowner (Variables|Default|GetUseDuration)))))

(fn PlayerReloadAbility
  (bind _playerowner (Variables|Default|GetPlayerOwner))
  (Utilities|IsValid _playerowner
    (:Is%20Valid
      (Default|ReloadAbility _playerowner (Variables|Default|GetReloadDuration))
      (Default|ServerSetIsUsingAbility (Variables|Default|GetPlayerOwner) false))))

(fn SetVFXVisibility
  (params (ShouldbeVisible :type Boolean)))

(fn OnRepIsVFXVisible
  (bind _playerowner (Variables|Default|GetPlayerOwner)
    (:then
      (Default|ServerSetAbilityVisibility _playerowner (Variables|Default|GetIsVFXVisible)))
    (:else)))

(fn NotifyAnimation)

(fn GetBasePlayerController
  (Variables|Default|GetBasePlayerController
    (:then
      _)
    (:else
      (bind _aspc_base_player_controller (Utilities|Casting|CastToPC_BasePlayerController (Game|GetPlayerController 0)))
      (Variables|Default|SetBasePlayerController _aspc_base_player_controller)))
  (return (Variables|Default|GetBasePlayerController)))