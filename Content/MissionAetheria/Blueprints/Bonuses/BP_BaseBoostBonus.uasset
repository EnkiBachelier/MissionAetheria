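; Base pickup actor for timed boost bonuses that modify a playable character's data.
; On BeginPlay it looks up its boost type in the bonuses DataTable for the effect duration, then destroys itself after a show delay if the row exists.
; Box overlap by a playable character passes the boost type, multiplier, duration and divide flag to that player controller's ServerBoostCharacterData.
; Init sets the boost type.
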(event OnComponentBeginOverlap(Box)
  (params (OverlappedComponent :type Primitive%20Component%20Object%20Reference) (OtherActor :type Actor%20Object%20Reference) (OtherComp :type Primitive%20Component%20Object%20Reference) (OtherBodyIndex :type Integer) (bFromSweep :type Boolean) (SweepResult :type Hit%20Result%20Structure%20%28by%20ref%29))
  (bind _asbp_base_playable_character (Utilities|Casting|CastToBP_BasePlayableCharacter OtherActor))
  (bind _aspc_base_player_controller (Utilities|Casting|CastToPC_BasePlayerController (Pawn|GetController _asbp_base_playable_character)))
  (Default|ServerBoostCharacterData _aspc_base_player_controller (Variables|Default|GetBoostType) (Variables|Default|GetMultiplier) (Variables|Default|GetDuration) (Variables|Default|GetShouldDivide) self))

(event EventBeginPlay
  (bind _returnvalue (Utilities|GetDataTableRow "/Game/MissionAetheria/Datatables/DataTable_Bonuses.DataTable_Bonuses" (Utilities|String|StringToName (Utilities|String|EnumtoString (Variables|Default|GetBoostType))))
    (:then
      (Variables|Default|SetDuration (.duration _returnvalue))
      (Utilities|FlowControl|Delay (Variables|Default|GetShowDuration))
      (Actor|DestroyActor))))

(fn ConstructionScript)

(fn Init
  (params (BoostType :type Enum_CharacterBoostType%20Enum :default "NewEnumerator0"))
  (Variables|Default|SetBoostType BoostType))