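; Sniper rifle weapon that extends a parent weapon class with penetrating hitscan shots.
; ShootBullet runs a multi line trace from the player pawn's camera, damaging IDamageable hits up to MaxPassesThrough, with base damage divided by each target's hit order.
; Damage, muzzle flash and Wwise shoot and reload sounds go through server calls on the player's controller or owner.
; The muzzle VFX is switched off at BeginPlay and toggled through a visibility override.
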(event EventBeginPlay
  (Default|ServerShowMuzzleShotVFX (CallFunction|GetBasePlayerController) "NewEnumerator4" false)
  (|CallParentFunction))

(fn ConstructionScript
  (|CallParentFunction))

(fn ShootBullet
  (bind _baseplayercontroller (CallFunction|GetBasePlayerController))
  (bind _playablecharacter (Default|GetPlayerPawn _baseplayercontroller))
  (|CallParentFunction)
  (Utilities|IsValid _playablecharacter
    (:Is%20Valid
      (Default|ServerPlaySfx (Variables|Default|GetPlayerOwner) "/Game/WwiseAudio/Events/Default_Work_Unit/SFX_Character/Weapons/Sniper/Play_Precision_Riffle_Shoot.Play_Precision_Riffle_Shoot" _playablecharacter)
      (bind _outhits (Default|CameraMultiLineTrace _playablecharacter (Variables|Default|GetmaxBulletDistance)))
      (Default|ServerShowMuzzleShotVFX (CallFunction|GetBasePlayerController) "NewEnumerator4" true)
      (LocalVariables|SetNbTouch 0)
      (for _array_element _outhits
        (bind _asidamageable (Utilities|Casting|CastToIDamageable (.HitActor (Collision|BreakHitResult _array_element))))
        (if (< (LocalVariables|GetNbTouch) (Variables|Default|GetMaxPassesThrough))
          (Default|ServerDealDamage (CallFunction|GetBasePlayerController) (/ (Variables|Default|GetAmountDamage) (+ (LocalVariables|GetNbTouch) 1)) _asidamageable false false (Variables|Default|GetPlayerOwner))
          (Math|Integer|IncrementInt (LocalVariables|GetNbTouch)))))))

(fn SetMuzzleShotVFXVisibility
  (params (IsActive :type Boolean))
  (bind _muzzleshot (Variables|Default|GetMuzzleShot))
  (if IsActive
    (Components|Activation|Activate _muzzleshot true)
    (else
      (Components|Activation|Deactivate _muzzleshot)))
  (|CallParentFunction false))

(fn Reload
  (|CallParentFunction)
  (Default|ServerPlaySfx (Variables|Default|GetPlayerOwner) "/Game/WwiseAudio/Events/Default_Work_Unit/SFX_Character/Weapons/Sniper/Play_Precision_Riffle_Reload.Play_Precision_Riffle_Reload" (Variables|Default|GetBasePlayerController)))