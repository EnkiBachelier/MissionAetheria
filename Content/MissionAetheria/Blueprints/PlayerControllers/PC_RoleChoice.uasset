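; Player controller for the role choice phase, relaying role selection and confirmation between players and the role-choice game state.
; Server events forward to multicasts that update GS_RoleChoice and switch input mode; opening role choice also shows the mouse cursor.
; Confirming a role also triggers a voiceline on the player character at index 0.
; Helper getters cast to the RoleChoice classes and game instance, caching all but the player state.
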(event Custom|Server_ModifyRoleState
  (params (role :type Enum_CharacterRoles%20Enum :default "NewEnumerator5") (player :type Struct%20Player%20Structure))
  ;[1 1 1] Modify Role State
  (CallFunction|MulticastModifyRoleState role player))

(event Custom|Multicast_CloseChoosingRole
  ;[1 1 1] Close Choosing Role
  (Input|SetInputModeGameOnly self false))

(event Custom|Server_OpenChoosingRole
  ;[1 1 1] Open Choosing Role
  (CallFunction|MulticastOpenChoosingRole))

(event Custom|Multicast_OpenChoosingRole
  ;[1 1 1] Open Choosing Role
  (Input|SetInputModeGameOnly self false)
  (Variables|Default|SetbShowMouseCursor true))

(event Custom|Multicast_ConfirmRole
  (params (Role :type Enum_CharacterRoles%20Enum :default "NewEnumerator5") (IsConfirm? :type Boolean))
  ;[1 1 1] ConfirmRole
  (Default|ConfirmRole (CallFunction|GetGameState) Role IsConfirm?))

(event Custom|Server_ConfirmRole
  (params (Role :type Enum_CharacterRoles%20Enum :default "NewEnumerator5") (IsConfirm? :type Boolean))
  (bind _playercharacter (CallFunction|GetPlayerCharacter))
  ;[1 1 1] ConfirmRole
  (CallFunction|MulticastConfirmRole Role IsConfirm?)
  (if IsConfirm?
    (Default|ServerPlayVoiceline _playercharacter _playercharacter "NewEnumerator1" Role "NewEnumerator1")))

(event Custom|Multicast_ModifyRoleState
  (params (role :type Enum_CharacterRoles%20Enum :default "NewEnumerator5") (player :type Struct%20Player%20Structure))
  ;[1 1 1] Modify Role State
  (Default|ModifyRoleState (CallFunction|GetGameState) role 0 player)
  (Input|SetInputModeUIOnly self 0 "DoNotLock" false))

(event Custom|Server_CloseChoosingRole
  ;[1 1 1] Close Choosing Role
  (CallFunction|MulticastCloseChoosingRole))

(fn ConstructionScript)

(fn ChangeRoleState
  (params (InRole :type Enum_CharacterRoles%20Enum :default "NewEnumerator5"))
  (CallFunction|ServerModifyRoleState InRole (Variables|/Game/MissionAetheria/Blueprints/PlayerStates/PS_BaseMissionAetheria.PS_BaseMissionAetheria_C|GetPlayer (CallFunction|GetPlayerState))))

(fn GetGameState
  (Utilities|IsValid (Variables|Default|GetGameState)
    (:Is%20Valid
      _)
    (:Is%20Not%20Valid
      (bind _asgs_role_choice (Utilities|Casting|CastToGS_RoleChoice (Game|GetGameState)))
      (Variables|Default|SetGameState _asgs_role_choice)))
  (return (Variables|Default|GetGameState)))

(fn GetPlayerState
  (bind _asps_role_choice (Utilities|Casting|CastToPS_RoleChoice (Variables|GetPlayerState)))
  (return _asps_role_choice))

(fn GetGameInstance
  (Utilities|IsValid (Variables|Default|GetGameInstance)
    (:Is%20Valid
      (return (Variables|Default|GetGameInstance)))
    (:Is%20Not%20Valid
      (bind _asgi_mission_aetheria (Utilities|Casting|CastToGI_MissionAetheria (Game|GetGameInstance)))
      (bind _output_get (Variables|Default|SetGameInstance _asgi_mission_aetheria))
      (return _output_get))))

(fn GetPlayerCharacter
  (Variables|Default|GetPlayerCharacter
    (:then
      _)
    (:else
      (bind _asbp_player_role_choice (Utilities|Casting|CastToBP_Player_RoleChoice (Game|GetPlayerCharacter 0)))
      (Variables|Default|SetPlayerCharacter _asbp_player_role_choice)))
  (return (Variables|Default|GetPlayerCharacter)))