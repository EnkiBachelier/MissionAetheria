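; Active ability for the hacked tank that throws out a hacking grenade and raises a shield.
; When the animation notify fires on the locally controlled owner, it server-spawns BP_HackingGrenade, then after a short delay flags the shield VFX visible and plays its sound.
; It reloads once the shield's duration elapses.
; The shield is a BP_Shield child actor, cast and cached on first access and disabled at BeginPlay.
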(event Custom|OnAbilitiesUsed
  (bind _playerowner (Variables|Default|GetPlayerOwner)
    (:then
      (Default|ServerSpawnActor _playerowner "/Game/MissionAetheria/Blueprints/Throwables/BP_HackingGrenade.BP_HackingGrenade_C" (Math|Transform|MakeTransform (Transformation|GetActorLocation) (Transformation|GetActorRotation)))
      (Utilities|FlowControl|Delay 0.5)
      (Variables|Default|SetIsVFXVisible true)
      (Default|ServerPlaySfx (Variables|Default|GetPlayerOwner) "/Game/WwiseAudio/Events/Default_Work_Unit/SFX_Character/Abilitys/Hacker/Play_SFX_SHIELD.Play_SFX_SHIELD" (Variables|Default|GetBasePlayerController))
      (CallFunction|PlayerUseAbility)
      (Utilities|FlowControl|Delay (Variables|Default|GetUseDuration))
      (CallFunction|OnReload))
    (:else)))

(event EventBeginPlay
  (CallFunction|SetVFXVisibility false)
  (Variables|Default|SetUseDuration (Variables|/Game/MissionAetheria/Blueprints/Abilities/Active/BP_Shield.BP_Shield_C|GetDuration (CallFunction|GetShield))))

(fn ConstructionScript
  (|CallParentFunction))

(fn Use
  (|CallParentFunction))

(fn GetShield
  (Variables|Default|GetShield
    (:then
      (return (Variables|Default|GetShield)))
    (:else
      (bind _asbp_shield (Utilities|Casting|CastToBP_Shield (Variables|/Script/Engine.ChildActorComponent|GetChildActor (Variables|Default|GetBP_Shield)))
        (:then
          (Variables|Default|SetShield _asbp_shield)
          (return (Variables|Default|GetShield)))
        (:CastFailed
          (Development|PrintString "BP_HackedTank | Cast to BP_Shield failed !" true true "(R=1.000000,G=0.000000,B=0.000000,A=1.000000)"))))))

(fn SetVFXVisibility
  (params (ShouldbeVisible :type Boolean))
  (Default|SetEnable (CallFunction|GetShield) ShouldbeVisible))

(fn NotifyAnimation
  (if (Pawn|IsLocallyControlled (Variables|Default|GetPlayerOwner))
    (CallFunction|OnAbilitiesUsed)))