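; Medic playable character, a child of a shared character base that sets its data and registers six canisters at BeginPlay.
; Init links the BP_Medic child actor to the right and left pistol child actors.
; A server event relays to a multicast that calls the ability VFX visibility function on each pistol.
; GetPistols lazily caches the pistols found in the weapon array.
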(event Custom|Multicast_ShowMedicVFXAbility
  (for _array_element (CallFunction|GetPistols)
    (Default|SetAbilityVFXVisibility _array_element)))

(event Custom|Server_ShowMedicVFXAbility
  (CallFunction|MulticastShowMedicVFXAbility))

(event EventBeginPlay
  (CallFunction|SetData "NewEnumerator1")
  (|CallParentFunction)
  (for _array_element (Utilities|Array|MakeArray (Variables|Default|GetCan_5) (Variables|Default|GetCan_4) (Variables|Default|GetCan_3) (Variables|Default|GetCan_2) (Variables|Default|GetCan_1) (Variables|Default|GetCan_0))
    (CallFunction|AddCannistertotheArray _array_element)))

(fn ConstructionScript
  (|CallParentFunction))

(fn Init
  (|CallParentFunction)
  (bind _asbp_medic (Utilities|Casting|CastToBP_Medic (Variables|/Script/Engine.ChildActorComponent|GetChildActor (Variables|Default|GetBP_Medic))))
  (bind _asbp_pistol (Utilities|Casting|CastToBP_Pistol (Variables|/Script/Engine.ChildActorComponent|GetChildActor (Variables|Default|GetBP_Pistol_Right))))
  (Default|Init _asbp_medic _asbp_pistol)
  (bind _asbp_pistol_2 (Utilities|Casting|CastToBP_Pistol (Variables|/Script/Engine.ChildActorComponent|GetChildActor (Variables|Default|GetBP_Pistol_Left))))
  (Default|Init _asbp_medic _asbp_pistol_2))

(fn GetPistols
  (if (Utilities|Array|IsNotEmpty (Variables|Default|GetPistols))
    _
    (else
      (for _array_element (Variables|Default|GetWeapon)
        (bind _asbp_pistol (Utilities|Casting|CastToBP_Pistol _array_element))
        (Utilities|Array|AddUnique (Variables|Default|GetPistols) _asbp_pistol))))
  (return (Variables|Default|GetPistols)))