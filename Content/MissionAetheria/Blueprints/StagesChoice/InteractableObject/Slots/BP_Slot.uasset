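; BP_Slot is an interactable level slot in the stage-choice area, showing a stage info panel for a data table row and its completion state from the game instance.
; Sphere overlaps toggle the player's info button and, on authority, ask the player to activate the panel based on others present.
; RepNotify variables drive panel open, delayed hide and front/back view.
; First interaction fires OnStartLevel; second requests a panel flip through the player controller.
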(event Custom|OnIsPanelVisibleSet
  (if (Variables|Default|GetIsPanelVisible)
    (Rendering|SetVisibility (Variables|Default|GetWidget) true false)
    (Default|OpenPanel (CallFunction|GetWidget))
    (else
      (Default|ClosePanel (CallFunction|GetWidget))
      (Utilities|FlowControl|Delay 0.5)
      (Rendering|SetVisibility (Variables|Default|GetWidget) false false))))

(event EventBeginPlay
  ;[0.03646 0.03646 0.03646] BeginPlay
  (bind _asgi_mission_aetheria (Utilities|Casting|CastToGI_MissionAetheria (Game|GetGameInstance)))
  (Default|InitUI (CallFunction|GetWidget) (Utilities|Array|ContainsItem (Variables|/Game/MissionAetheria/Blueprints/GameInstance/GI_MissionAetheria.GI_MissionAetheria_C|GetCompletedLevelsRowName _asgi_mission_aetheria) (Variables|Default|GetDataTableRowToLoad)) (Variables|Default|GetDataTableRowToLoad)))

(event EventEndPlay
  (params (EndPlayReason :type EEndPlayReason%20Enum :default "Destroyed"))
  ;[0.04167 0.04167 0.04167] EndPlay
  (EventDispatchers|UnbindallEventsfromOnStartLevel))

(fn ConstructionScript
  (|CallParentFunction))

(fn ActivePanel
  (params (isActive :type Boolean))
  (if (!= isActive (Variables|Default|GetIsPanelVisible))
    (Development|PrintString (Utilities|String|ToString(Boolean) isActive))
    (bind _output_get (Variables|Default|SetIsPanelVisible isActive))
    (return _output_get)
    (else
      (return false))))

(fn BeginOverlap
  (params (Player :type BP%20Player%20Stages%20Choice%20Object%20Reference))
  (Default|ActiveInfoButton Player true)
  (if (Variables|Default|GetIsPanelVisible)
    _
    (else
      (Variables|Default|SetisPanelViewFront true)
      (Default|SetView (CallFunction|GetWidget) (Variables|Default|GetisPanelViewFront))))
  (if (Ability|HasAuthority Player)
    (Default|ServerActiveSlotPanel Player true self (> (Utilities|Array|Length (Collision|GetOverlappingActors (Variables|Default|GetSphere) "/Game/MissionAetheria/Blueprints/Player/BP_Player_StagesChoice.BP_Player_StagesChoice_C" :!class /Script/Engine.PrimitiveComponent)) 1))))

(fn EndOverlap
  (params (Player :type BP%20Player%20Stages%20Choice%20Object%20Reference))
  (Default|ActiveInfoButton Player false)
  (if (Ability|HasAuthority Player)
    (Default|ServerActiveSlotPanel Player false self (> (Utilities|Array|Length (Collision|GetOverlappingActors (Variables|Default|GetSphere) "/Game/MissionAetheria/Blueprints/Player/BP_Player_StagesChoice.BP_Player_StagesChoice_C" :!class /Script/Engine.PrimitiveComponent)) 0))))

(fn GetWidget
  (Utilities|IsValid (Variables|Default|GetUIStagePanel)
    (:Is%20Valid
      _)
    (:Is%20Not%20Valid
      (bind _aswbp_stage_panel (Utilities|Casting|CastToWBP_StagePanel (UserInterface|GetWidget (Variables|Default|GetWidget))))
      (Variables|Default|SetUIStagePanel _aswbp_stage_panel)))
  (return (Variables|Default|GetUIStagePanel)))

(fn OnRepIsPanelVisible
  (CallFunction|OnIsPanelVisibleSet))

(fn FirstInteraction
  (params (player :type BP%20Player%20Stages%20Choice%20Object%20Reference))
  (Default|CallOnStartLevel self))

(fn SecondInteraction
  (params (Player :type BP%20Player%20Stages%20Choice%20Object%20Reference))
  (Default|ServerTurnPanel (Variables|/Game/MissionAetheria/Blueprints/Player/BP_Player_StagesChoice.BP_Player_StagesChoice_C|GetPlayerController Player) (not (Variables|Default|GetisPanelViewFront)) self))

(fn OnRepIsPanelViewFront
  (Default|SetView (CallFunction|GetWidget) (Variables|Default|GetisPanelViewFront)))