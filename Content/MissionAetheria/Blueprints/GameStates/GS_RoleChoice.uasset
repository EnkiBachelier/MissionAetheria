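; Game State for the role selection phase, tracking each player's chosen role and confirmation.
; On BeginPlay the server restores the choices array from the Game Instance, or seeds it unconfirmed from the player list.
; Functions add players by unique UserID, reject roles others hold, lock confirmed choices, and push role changes to each PS_RoleChoice.
; SavePlayersTab writes the array back to the Game Instance and has each Player State save.
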(event EventBeginPlay
  (bind _gameinstance (CallFunction|GetGameInstance))
  (bind _playersrolechoice (Variables|/Game/MissionAetheria/Blueprints/GameInstance/GI_MissionAetheria.GI_MissionAetheria_C|GetPlayersRoleChoice _gameinstance))
  (|CallParentFunction)
  (if (Networking|IsServer)
    (if (> (Utilities|Array|Length _playersrolechoice) 0)
      (bind _output_get (Variables|Default|SetPlayersRolesChoices _playersrolechoice))
      (else
        (Utilities|Array|Clear (Variables|Default|GetPlayersRolesChoices))
        (for _array_element (Variables|/Game/MissionAetheria/Blueprints/GameInstance/GI_MissionAetheria.GI_MissionAetheria_C|GetPlayers (CallFunction|GetGameInstance))
          (Utilities|Array|AddUnique (Variables|Default|GetPlayersRolesChoices) (Utilities|Struct|MakeStruct_PlayerRolesChoice _array_element false)))))))

(fn ConstructionScript)

(fn ModifyRoleState
  (params (Role :type Enum_CharacterRoles%20Enum :default "NewEnumerator5") (PlayerState :type PS%20Role%20Choice%20Object%20Reference) (player :type Struct%20Player%20Structure))
  (for (_array_element _array_index) (Variables|Default|GetPlayersRolesChoices)
    (if (not (.IsConfirm (Utilities|Struct|BreakStruct_PlayerRolesChoice _array_element)))
      (if (== (.name (.Player (Utilities|Struct|BreakStruct_PlayerRolesChoice _array_element))) (.Name (Utilities|Struct|BreakStruct_Player player)))
        (for _array_element_2 (Variables|Default|GetPlayersRolesChoices)
          (if (!= (.name (.player _array_element_2)) (.name player))
            (if (Utilities|Enum|Equal(Enum) (.role (.player _array_element_2)) Role)
              (LocalVariables|SetRoleAlreadyTaken true))))
        (if (not (LocalVariables|GetRoleAlreadyTaken))
          (Utilities|Array|SetArrayElem (Variables|Default|GetPlayersRolesChoices) _array_index (Utilities|Struct|MakeStruct_PlayerRolesChoice (Utilities|Struct|MakeStruct_Player (.name (.Player (Utilities|Struct|BreakStruct_PlayerRolesChoice _array_element))) (.texture (.Player (Utilities|Struct|BreakStruct_PlayerRolesChoice _array_element))) Role (.playerstate (.Player (Utilities|Struct|BreakStruct_PlayerRolesChoice _array_element))) "" "(GamePlayedCount_24_14712699483358EB0DE519A19778F9C0=0.000000,LosesCount_25_A97B0A2149FE197864C76D9A033A1535=0.000000,WinsCount_26_DF53EB69415FC1E198B1D3A77B6E2C47=0.000000,TimePlayed_27_952AD6384EF515644A55D591B3CAB726=0.000000,TimeUsedHacker_28_148B17EB4E02539A59B69D87DB60416B=0.000000,TimeUsedHealer_29_27FDC7FC4F8CBFDE1B631887DD28FEF2=0.000000,TimeUsedPilote_30_98D7B2524A7D0907C76A1EAC022D83CA=0.000000,TimeUsedPyromaniac_31_341273A64513B0D71204DE9A296560E5=0.000000,TimeUsedSniper_32_A58766A24D6575B96C876D9086520644=0.000000)") false))
          (CallFunction|UpdatePlayersStates))))))

(fn ConfirmRole
  (params (Role :type Enum_CharacterRoles%20Enum :default "NewEnumerator5") (ISConfirm? :type Boolean))
  (for (_array_element _array_index) (Variables|Default|GetPlayersRolesChoices)
    (if (Utilities|Enum|Equal(Enum) (.role (.player _array_element)) Role)
      (Utilities|Array|SetArrayElem (Variables|Default|GetPlayersRolesChoices) _array_index (Utilities|Struct|MakeStruct_PlayerRolesChoice (.player (Utilities|Array|Get(acopy) (Variables|Default|GetPlayersRolesChoices) _array_index)) ISConfirm?)))))

(fn AddPlayerRoleChoice
  (params (player :type Struct%20Player%20Roles%20Choice%20Structure%20%28by%20ref%29))
  (bind _player (Utilities|Struct|BreakStruct_PlayerRolesChoice player))
  (bind _array_element (Utilities|Array|ForEachLoopwithBreak (Variables|Default|GetPlayersRolesChoices) :!label _label)
    (:LoopBody
      (bind _output_get (LocalVariables|SetIsUnique (Utilities|Enum|NotEqual(Enum) (.userid (.player _array_element)) (.userid _player))))
      (if (not _output_get)
        (goto _label Break)))
    (:Completed
      (if (and (Utilities|Enum|NotEqual(Enum) (Utilities|String|ToString(Name) (.name _player)) "None") (LocalVariables|GetIsUnique))
        (Utilities|Array|AddUnique (Variables|Default|GetPlayersRolesChoices) player)))))

(fn UpdatePlayersStates
  (for _array_element (Variables|Default|GetPlayersRolesChoices)
    (bind _asps_role_choice (Utilities|Casting|CastToPS_RoleChoice (.PlayerState (Utilities|Struct|BreakStruct_Player (.player _array_element)))))
    (Variables|/Game/MissionAetheria/Blueprints/PlayerStates/PS_BaseMissionAetheria.PS_BaseMissionAetheria_C|SetPlayer _asps_role_choice (.player _array_element))))

(fn SavePlayersTab
  (bind _output_get (Variables|/Game/MissionAetheria/Blueprints/GameInstance/GI_MissionAetheria.GI_MissionAetheria_C|SetPlayersRoleChoice (CallFunction|GetGameInstance) (Variables|Default|GetPlayersRolesChoices)))
  (for _array_element _output_get
    (bind _asps_role_choice (Utilities|Casting|CastToPS_RoleChoice (.PlayerState (Utilities|Struct|BreakStruct_Player (.player _array_element)))))
    (Variables|/Game/MissionAetheria/Blueprints/PlayerStates/PS_BaseMissionAetheria.PS_BaseMissionAetheria_C|SetPlayer _asps_role_choice (.player _array_element))
    (Default|SavePlayer _asps_role_choice)))