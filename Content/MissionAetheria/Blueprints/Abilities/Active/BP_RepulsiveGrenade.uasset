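; Active ability Blueprint for a repulsive grenade that spawns a BP_SniperGrenade when used.
; An animation notify triggers the use only on the locally controlled player.
; With a valid owner, it requests a server-side spawn at the ability actor's transform, registers the use, then starts reload after the use duration.
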(event Custom|OnAbilitieUsed
  ;[1 1 1] Spawn grenade
  (bind _playerowner (Variables|Default|GetPlayerOwner)
    (:then
      (Default|ServerSpawnActor _playerowner "/Game/MissionAetheria/Blueprints/Throwables/BP_SniperGrenade.BP_SniperGrenade_C" (Transformation|GetActorTransform))
      (CallFunction|PlayerUseAbility)
      (Utilities|FlowControl|Delay (Variables|Default|GetUseDuration))
      (CallFunction|OnReload))
    (:else)))

(fn ConstructionScript
  (|CallParentFunction))

(fn NotifyAnimation
  (if (Pawn|IsLocallyControlled (Variables|Default|GetPlayerOwner))
    (CallFunction|OnAbilitieUsed)))