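; Rifle weapon Blueprint that extends a parent weapon's shoot, reload and muzzle-flash behavior.
; Shooting runs a hitscan trace from the player pawn's camera and sends damage for IDamageable hits through the player controller's server call.
; Wwise fire and reload sounds and muzzle VFX requests also go through server calls, with the flash switched off on BeginPlay.
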(event Custom|OnFireBullets_1)

(event Custom|OnReload_1)

(event EventBeginPlay
  (Default|ServerShowMuzzleShotVFX (CallFunction|GetBasePlayerController) "NewEnumerator3" false)
  (|CallParentFunction))

(fn ConstructionScript
  (|CallParentFunction))

(fn ShootBullet
  (bind _baseplayercontroller (CallFunction|GetBasePlayerController))
  (bind _playablecharacter (Default|GetPlayerPawn _baseplayercontroller))
  (|CallParentFunction)
  (Utilities|IsValid _playablecharacter
    (:Is%20Valid
      (Default|ServerPlaySfx (Variables|Default|GetPlayerOwner) "/Game/WwiseAudio/Events/Default_Work_Unit/SFX_Character/Weapons/Hacker/Play_Tek_riffle.Play_Tek_riffle" _baseplayercontroller)
      (Default|ServerShowMuzzleShotVFX _baseplayercontroller "NewEnumerator3" true)
      (bind _outhit (Default|CameraLineTrace _playablecharacter (Variables|Default|GetMaxBulletDistance)))
      (bind _asidamageable (Utilities|Casting|CastToIDamageable (.hitactor _outhit)))
      (Default|ServerDealDamage (CallFunction|GetBasePlayerController) (Variables|Default|GetAmountDamage) _asidamageable false false (Variables|Default|GetPlayerOwner)))))

(fn SetMuzzleShotVFXVisibility
  (params (IsActive :type Boolean))
  (bind _muzzleshot (Variables|Default|GetMuzzleShot))
  (if IsActive
    (Components|Activation|Activate _muzzleshot true)
    (else
      (Components|Activation|Deactivate _muzzleshot)))
  (|CallParentFunction IsActive))

(fn Reload
  (|CallParentFunction)
  (Default|ServerPlaySfx (Variables|Default|GetPlayerOwner) "/Game/WwiseAudio/Events/Default_Work_Unit/SFX_Character/Weapons/Hacker/Play_Riffle_tek_reload.Play_Riffle_tek_reload" (Variables|Default|GetBasePlayerController)))