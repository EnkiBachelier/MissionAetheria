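; BP_AI_Range is an AI Blueprint, apparently for a ranged unit, that supplies an attack range based on the target player.
; GetAttackRange gives the Pilot character a long range when per-axis X and Y offset checks pass, a medium one otherwise, and other classes a shorter one.
; The offset helper's tolerance comparison appears unconnected to any output.
; Auto-generated hit and overlap functions only print debug messages, and the default events are disabled.
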(event EventBeginPlay
  (|CallParentFunction) ; This node is disabled and will not be called.\nDrag off pins to build functionality.
)

(event Collision|EventActorBeginOverlap
  (params (OtherActor :type Actor%20Object%20Reference)))

(event EventTick
  (params (DeltaSeconds :type Float%20%28single-precision%29))
  (|CallParentFunction DeltaSeconds) ; This node is disabled and will not be called.\nDrag off pins to build functionality.
)

(fn ConstructionScript
  (|CallParentFunction))

(fn BPAIRangeAutoGenFunc
  (params (HitComponent :type Primitive%20Component%20Object%20Reference) (OtherActor :type Actor%20Object%20Reference) (OtherComp :type Primitive%20Component%20Object%20Reference) (NormalImpulse :type Vector) (Hit :type Hit%20Result%20Structure%20%28by%20ref%29))
  (Development|PrintString (Utilities|String|Append "Hit other actor " (Utilities|GetDisplayName OtherActor)) true true "(R=0.293095,G=0.000000,B=1.000000,A=1.000000)" 1e+01)
  (return))

(fn BPAIRangeAutoGenFunc1
  (params (OverlappedComponent :type Primitive%20Component%20Object%20Reference) (OtherActor :type Actor%20Object%20Reference) (OtherComp :type Primitive%20Component%20Object%20Reference) (OtherBodyIndex :type Integer) (bFromSweep :type Boolean) (SweepResult :type Hit%20Result%20Structure%20%28by%20ref%29))
  (Development|PrintString (Utilities|String|Append "Hit other actor " (Utilities|GetDisplayName OtherActor)) true true "(R=0.942750,G=1.000000,B=0.000000,A=1.000000)" 1e+01)
  (return))

(fn GetAttackRange
  (params (Player :type BP%20Base%20Playable%20Character%20Object%20Reference))
  (bind _returnvalue (Transformation|GetActorLocation Player))
  (bind _returnvalue_2 (Transformation|GetActorLocation))
  (if (== (Utilities|GetClass Player) "/Game/MissionAetheria/Blueprints/Player/PlayableCharacters/BP_PlayableCharacter_Pilot.BP_PlayableCharacter_Pilot_C")
    (if (and (Utilities|SubstractValueinRangeDistancePilote (.x _returnvalue_2) (.x _returnvalue)) (Utilities|SubstractValueinRangeDistancePilote (.y _returnvalue_2) (.y _returnvalue)))
      (return 2.5e+03)
      (else
        (return 1e+03)))
    (else
      (return 8e+02))))