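; BP_AI_Melee is the melee AI Blueprint, providing a bone-based attack that damages playable characters.
; Attack takes an animation index, looks up the matching bone name and runs a zero-length sphere trace at that bone's world location on the Camera channel.
; A hit actor derived from BP_BasePlayableCharacter receives DealDamageMessage with the damage amount.
; The event graph holds only disabled nodes, so Attack is the only logic here.
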(event EventBeginPlay
  (|CallParentFunction) ; This node is disabled and will not be called.\nDrag off pins to build functionality.
)

(event Collision|EventActorBeginOverlap
  (params (OtherActor :type Actor%20Object%20Reference)))

(event EventTick
  (params (DeltaSeconds :type Float%20%28single-precision%29))
  (|CallParentFunction DeltaSeconds) ; This node is disabled and will not be called.\nDrag off pins to build functionality.
)

(fn ConstructionScript
  (|CallParentFunction))

(fn Attack
  (params (IndexAnimAttack :type Integer))
  (bind _mesh (Variables|Character|GetMesh))
  (bind _boneattacknamed (Variables|Default|GetBoneAttackNamed))
  (bind _output (Utilities|Array|Get(acopy) _boneattacknamed IndexAnimAttack))
  (bind _returnvalue (Transformation|GetBoneTransform _mesh _output "RTS_World"))
  (if (< IndexAnimAttack (Utilities|Array|Length (Variables|Default|GetBoneAttackNamed)))
    (bind (_outhit _returnvalue_2) (Collision|SphereTraceByChannel (.location _returnvalue) (.location _returnvalue) 2e+01 "TraceTypeQuery2" false 0 "None"))
    (if (and _returnvalue_2 (Utilities|ClassIsChildOf (Utilities|GetClass (.HitActor (Collision|BreakHitResult _outhit))) "/Game/MissionAetheria/Blueprints/Player/BP_BasePlayableCharacter.BP_BasePlayableCharacter_C"))
      (Class|IDamageable|DealDamage(Message) (.HitActor (Collision|BreakHitResult _outhit)) (CallFunction|GetDamageAmount) "NewEnumerator1"))))