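; BP_Shield is the active shield ability that the hacker tank triggers through its ability input.
; It starts with the Niagara shield effect off, and SetEnable toggles that effect together with the shield mesh's collision between query-only and none.
; When enabled, it waits for a Duration delay and then calls SetEnable again to switch itself off.
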(event Custom|SetEnable
  (params (IsEnable :type Boolean))
  (bind _sm_shield_02 (Variables|Default|GetSM_Shield_02))
  (bind _ns_shield (Variables|Default|GetNS_Shield))
  ;[1 1 1] SetEnable
  (if IsEnable
    (Components|Activation|Activate _ns_shield true)
    (Collision|SetCollisionEnabled _sm_shield_02 "QueryOnly")
    (Utilities|FlowControl|Delay (Variables|Default|GetDuration))
    (CallFunction|SetEnable false)
    (else
      (Components|Activation|Deactivate _ns_shield)
      (Collision|SetCollisionEnabled _sm_shield_02 "NoCollision"))))

(event EventBeginPlay
  ;[1 1 1] Init Shield
  (Components|Activation|Deactivate (Variables|Default|GetNS_Shield)))

(fn ConstructionScript)