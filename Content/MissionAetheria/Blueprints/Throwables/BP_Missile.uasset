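; BP_Missile is a reusable throwable missile projectile, toggled by SetinUse, which switches visibility, collision and velocity and moves it away when disabled.
; When enabled, it flies forward, ignores its owner and broadcasts OnKilled after a timed lifetime.
; Overlaps with non-ignored classes play a Wwise sound and, if enabled, report the hit through the player controller's ServerOnMissileHit.
; OnMissileHit fires the radial impulse and broadcasts OnKilled.
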(event OnComponentBeginOverlap(Capsule)
  (params (OverlappedComponent :type Primitive%20Component%20Object%20Reference) (OtherActor :type Actor%20Object%20Reference) (OtherComp :type Primitive%20Component%20Object%20Reference) (OtherBodyIndex :type Integer) (bFromSweep :type Boolean) (SweepResult :type Hit%20Result%20Structure%20%28by%20ref%29))
  (if (not (Utilities|Array|ContainsItem (Variables|Default|GetActorToIgnore) (Utilities|GetClass OtherActor)))
    (Class|AkGameplayStatics|PostEventatLocation "/Game/WwiseAudio/Events/Default_Work_Unit/SFX_Character/Abilitys/Pilot/Play_SFX_war_plane_missiles.Play_SFX_war_plane_missiles" (Transformation|GetWorldLocation (Variables|Default|GetMissile)) "0, 0, 0")
    (if (Variables|Default|GetisEnabled)
      (Default|ServeronMissileHit (Variables|Default|GetplayerController) self (Variables|/Script/Engine.RadialForceComponent|GetRadius (Variables|Default|GetRadialForce))))))

(event EventBeginPlay
  (bind _aspc_base_player_controller (Utilities|Casting|CastToPC_BasePlayerController (Game|GetPlayerController 0)))
  (Variables|Default|SetplayerController _aspc_base_player_controller))

(event EventEndPlay
  (params (EndPlayReason :type EEndPlayReason%20Enum :default "Destroyed"))
  (EventDispatchers|UnbindallEventsfromOnKilled))

(event EventSetinUse
  (params (InUse :type Boolean))
  (bind _projectilemovement (Variables|Default|GetProjectileMovement))
  ;[1 1 1] Set In Use
  (bind _output_get (Variables|Default|SetisEnabled InUse))
  (Collision|SetCollisionEnabled (Variables|Default|GetCapsule) "QueryOnly")
  (Collision|SetActorEnableCollision _output_get)
  (Rendering|SetActorHiddenInGame (not _output_get))
  (if InUse
    (Variables|/Script/Engine.MovementComponent|SetVelocity _projectilemovement (* (Math|Rotator|GetRotationXVector (Transformation|GetActorRotation)) (Variables|Default|GetMissileSpeed)))
    (Collision|IgnoreActorwhenMoving (Variables|Default|GetMissile) (Components|GetOwner) true)
    (Utilities|FlowControl|Delay (Variables|Default|GettimeBeforeDelete))
    (Default|CallOnKilled self)
    (else
      (Variables|/Script/Engine.MovementComponent|SetVelocity _projectilemovement "0, 0, 0")
      (Transformation|SetActorLocation "-100.000000,-100.000000,-100.000000" false false) ; Hotfix to avoid a frame where the collision is still active
    )))

(fn ConstructionScript)

(fn OnMissileHit
  (Class|RadialForceComponent|FireImpulse (Variables|Default|GetRadialForce))
  (Default|CallOnKilled self))