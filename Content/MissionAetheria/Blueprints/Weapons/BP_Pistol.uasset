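; Pistol weapon Blueprint that extends a parent weapon with hitscan shooting, reload audio and muzzle and ability VFX.
; Shooting traces from the pawn's camera, deals damage to IDamageable hits and broadcasts OnEntityDamaged for the medic ability.
; Damage, sound and muzzle flash are routed through Server calls on the owning player or controller.
; Ability VFX activates on BeginPlay, and damage-event bindings are cleared on destruction.
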(event EventBeginPlay
  (Default|ServerShowMuzzleShotVFX (CallFunction|GetBasePlayerController) "NewEnumerator1" false)
  (CallFunction|SetAbilityVFXVisibility)
  (|CallParentFunction))

(event EventDestroyed
  (EventDispatchers|UnbindallEventsfromOnEntityDamaged))

(fn ConstructionScript
  (|CallParentFunction))

(fn ShootBullet
  (bind _amountdamage (Variables|Default|GetAmountDamage))
  ;[1 1 1] Shoot bullet
  (|CallParentFunction)
  (Default|ServerShowMuzzleShotVFX (CallFunction|GetBasePlayerController) "NewEnumerator1" true)
  (Default|ServerPlaySfx (Variables|Default|GetPlayerOwner) "/Game/WwiseAudio/Events/Default_Work_Unit/SFX_Character/Weapons/Medic/Play_Shoot_Pistol.Play_Shoot_Pistol" (Variables|Default|GetBasePlayerController))
  (bind _outhit (Default|CameraLineTrace (Default|GetPlayerPawn (CallFunction|GetBasePlayerController)) (Variables|Default|GetMaxBulletDistance)))
  (LocalVariables|SetHitActor (.hitactor _outhit))
  (bind _asidamageable (Utilities|Casting|CastToIDamageable (LocalVariables|GetHitActor)))
  (Default|ServerDealDamage (CallFunction|GetBasePlayerController) _amountdamage _asidamageable false false (Variables|Default|GetPlayerOwner))
  (Default|CallOnEntityDamaged _amountdamage) ; For the ability medic
)

(fn SetMuzzleShotVFXVisibility
  (params (IsActive :type Boolean))
  (bind _muzzleshot (Variables|Default|GetMuzzleShot))
  (if IsActive
    (Components|Activation|Activate _muzzleshot true)
    (else
      (Components|Activation|Deactivate _muzzleshot)))
  (|CallParentFunction false))

(fn Reload
  (|CallParentFunction)
  (Default|ServerPlaySfx (Variables|Default|GetPlayerOwner) "/Game/WwiseAudio/Events/Default_Work_Unit/SFX_Character/Weapons/Medic/Play_Reload_Pisto.Play_Reload_Pisto" (Variables|Default|GetBasePlayerController)))

(fn SetAbilityVFXVisibility
  (Components|Activation|Activate (Variables|Default|GetAbility) true))